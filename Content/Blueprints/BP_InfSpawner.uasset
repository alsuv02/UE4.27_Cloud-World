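; BP_InfSpawner is an actor that endlessly spawns BP_ArcherCharacterEnemy at its own location until the player dies.
; On BeginPlay it caches the player as BP_MainCharacterCW and starts a one-second looping timer, apparently bound to SpawnEnemy.
; Each SpawnEnemy call spawns an archer, then clears the timer if the player's IsDead flag is set, so the check follows the spawn.
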(event `self.ReceiveBeginPlay`
  ;[0 1 0.01344] Comment
  (bind _asbp_main_character_cw (cast `/Game/Blueprints/BP_MainCharacterCW` (`GameplayStatics.GetPlayerCharacter` 0)))
  (set `self.As Top Down Character` _asbp_main_character_cw)
  (bind _returnvalue (`KismetSystemLibrary.K2_SetTimerDelegate` (`|CreateDelegate` :!event `Spawn Enemy`) 1.0 true))
  (set `self.Handler` _returnvalue))

(event `Spawn Enemy`
  (`|SpawnActorFromClass` "/Game/Blueprints/Enemy/BP_ArcherCharacterEnemy.BP_ArcherCharacterEnemy_C" (`KismetMathLibrary.MakeTransform` (`self.K2_GetActorLocation`)) "Undefined" "OverrideRootScale" null null)
  (if (`/Game/Blueprints/BP_MainCharacterCW.IsDead` (`self.As Top Down Character`))
    (`KismetSystemLibrary.K2_ClearAndInvalidateTimerHandle` (`self.Handler`))))

(fn `UserConstructionScript`)