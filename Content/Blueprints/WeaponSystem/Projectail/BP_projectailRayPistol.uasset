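; Ray pistol projectile that draws its shot as a sphere stretched along Z and damages what it hits.
; Gated Tick logic lengthens the sphere by a Speed-based step for a short time, then applies one similar shrink step and closes the extension gate.
; When projectile movement stops, it applies damage to the hit actor, reports an AI damage-sense event and destroys the projectile.
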(event `self.ReceiveBeginPlay`
  (`parent.ReceiveBeginPlay`)
  (`self.ExtantionBegin`))

(event `self.ReceiveTick`
  (params (DeltaSeconds :type "Float (single-precision)"))
  (`parent.ReceiveTick` DeltaSeconds)
  (`self.ExtantionTick`)
  (`self.DecreaseTick`))

(event `ExtantionTick`
  (bind _sphere (`self.Sphere`))
  (bind _returnvalue (+ (`self.LifeTime`) (`self.Delta Seconds`)))
  ;[1 1 1] Comment
  (`/Engine/EditorBlueprintResources/StandardMacros.Gate` true :!label _label
    (:`Exit`
      (`SceneComponent.SetRelativeScale3D` _sphere (+ (`SceneComponent.RelativeScale3D` _sphere) (`KismetMathLibrary.MakeVector` 0.0 0.0 (/ (`self.Speed`) 3000.0))))
      (if (<= _returnvalue 0.3)
        (set `self.LifeTime` _returnvalue)
        (else
          (`self.DecreaseStart`)
          (`self.ExtantionStop`)
          (set `self.LifeTime` 0.0))))))

(event `ExtantionBegin`
  ;[1 1 1] Comment
  (goto _label :!via `Open`))

(event `ExtantionStop`
  ;[1 1 1] Comment
  (goto _label :!via `Close`))

(event `DecreaseStart`
  (bind _sphere (`self.Sphere`))
  (bind _returnvalue (+ (`self.LifeTime`) (`self.Delta Seconds`)))
  ;[1 1 1] Comment
  (`/Engine/EditorBlueprintResources/StandardMacros.Gate` true :!label _label_2
    (:`Exit`
      (`SceneComponent.SetRelativeScale3D` _sphere (- (`SceneComponent.RelativeScale3D` _sphere) (`KismetMathLibrary.MakeVector` 0.0 0.0 (/ (`self.Speed`) 3010.0))))
      (if (<= _returnvalue 1.0)
        (set `self.LifeTime` _returnvalue)))))

(event `DecreaseTick`
  ;[1 1 1] Comment
  (goto _label_2 :!via `Open`))

(event `DecreasStop`
  ;[1 1 1] Comment
  (goto _label_2 :!via `Close`))

(event `self.ProjectileMovement.OnProjectileStop`
  (params (ImpactResult :type "HitResult Structure (by ref)"))
  (bind (_bblockinghit _binitialoverlap _time _distance _location _impactpoint _normal _impactnormal _physmat _hitactor) (`GameplayStatics.BreakHitResult` ImpactResult))
  (bind _damage (`self.Damage`))
  ;[1 1 1] Comment
  (`GameplayStatics.ApplyDamage` _hitactor _damage null self "/Script/Engine.DamageType")
  (`AISense_Damage.ReportDamageEvent` _hitactor self _damage _location (0.0 0.0 0.0) "Damage")
  (`self.ProjDestroy`))

(fn `UserConstructionScript`
  (`parent.UserConstructionScript`))