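; Lightning pistol projectile that damages what it hits, then relaunches toward another enemy as a chain attack.
; On each projectile stop it applies damage, reports a damage event, and searches living BP_CharacterEnemyParent actors, excluding the one hit, by distance from the impact.
; Bounces off enemies divide damage and sphere scale by a growing counter.
; The projectile is destroyed at the bounce limit or when no target remains.
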(event `self.ReceiveTick`
  (params (DeltaSeconds :type "Float (single-precision)"))
  (`parent.ReceiveTick` DeltaSeconds))

(event `self.ProjectileMovement.OnProjectileStop`
  (params (ImpactResult :type "HitResult Structure (by ref)"))
  (bind (_bblockinghit _binitialoverlap _time _distance _location _impactpoint _normal _impactnormal _physmat _hitactor) (`GameplayStatics.BreakHitResult` ImpactResult))
  (bind _damage (`self.Damage`))
  (set `self.Hit Actor` _hitactor)
  (set `self.HitLocation` _location)
  (`GameplayStatics.ApplyDamage` (`self.Hit Actor`) _damage null self "/Script/Engine.DamageType")
  (`AISense_Damage.ReportDamageEvent` (`self.Hit Actor`) self _damage _location (0.0 0.0 0.0) "Damage")
  (`self.LookForEnemy`))

(event `LookForEnemy`
  ;[1 1 1] Comment
  (bind _outactors (`GameplayStatics.GetAllActorsOfClass` "/Game/Blueprints/Enemy/BP_CharacterEnemyParent.BP_CharacterEnemyParent_C"))
  (for _array_element _outactors
    (if (not (`/Game/Blueprints/Enemy/BP_CharacterEnemyParent.IsDead` _array_element))
      (`KismetArrayLibrary.Array_Add` (`self.Out Actors`) _array_element)))
  (`/Engine/EditorBlueprintResources/StandardMacros.IsValid` (`|GetArrayItem` (`self.Out Actors`))
    (:`Is Valid`
      (set `self.NewTarget` null)
      (for _array_element_2 (`self.Out Actors`)
        (if (== (`self.Hit Actor`) _array_element_2)
          _
          (elif (`self.IsFirstLoop`)
            (set `self.IsFirstLoop` false)
            (bind _returnvalue (`KismetMathLibrary.Vector_Distance` (`self.HitLocation`) (`self.K2_GetActorLocation` _array_element_2)))
            (set `self.Distance` _returnvalue :!label _label)
            (set `self.NewTarget` _array_element_2)
            (elif (< _returnvalue (`self.Distance`))
              (goto _label)))))
      (`KismetArrayLibrary.Array_Clear` (`self.Out Actors`))
      (`self.LaunchAgain`))
    (:`Is Not Valid`
      (`self.ProjDestroy`))))

(event `LaunchAgain`
  ;[1 1 1] запускаем вновь
  (`/Engine/EditorBlueprintResources/StandardMacros.IsValid` (`self.NewTarget`)
    (:`Is Valid`
      (`MovementComponent.SetUpdatedComponent` (`self.ProjectileMovement`) (`self.Sphere`))
      (set `MovementComponent.Velocity` (* (`KismetMathLibrary.GetDirectionUnitVector` (`self.HitLocation`) (`self.K2_GetActorLocation` (`self.NewTarget`))) (`self.Speed`)) (`self.ProjectileMovement`))
      (cast `/Game/Blueprints/Enemy/BP_CharacterEnemyParent` (`self.Hit Actor`))
      (`self.CounterUpdate`))
    (:`Is Not Valid`
      (`self.ProjDestroy`))))

(event `CounterUpdate`
  (bind _sphere (`self.Sphere`))
  (bind _relativescale3d_x (`KismetMathLibrary.BreakVector` (`SceneComponent.RelativeScale3D` _sphere)))
  (bind _returnvalue (/ _relativescale3d_x (`self.RestartCounter`)))
  ;[1 1 1] Comment
  (bind _result (`/Engine/EditorBlueprintResources/StandardMacros.IncrementFloat` (`self.RestartCounter`))
    (:`  `
      (if (>= _result 5.0)
        (`self.ProjDestroy`)
        (else
          (set `self.Damage` (/ (`self.Damage`) (`self.RestartCounter`)))
          (`SceneComponent.SetRelativeScale3D` _sphere (`KismetMathLibrary.MakeVector` _returnvalue _returnvalue _returnvalue)))))))

(fn `UserConstructionScript`
  (`parent.UserConstructionScript`))