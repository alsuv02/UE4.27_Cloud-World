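; Wight staff projectile whose scale and damage change over its short lifetime.
; On BeginPlay, after the parent logic, the SizeChage timeline drives uniform actor scale and recalculates Damage every update, then destroys the actor when finished.
; An inline note intends damage to fall from 6 to 1 as size shrinks, but the formula feeds Damage back into itself, so it compounds each update.
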(event `self.ReceiveBeginPlay`
  (`parent.ReceiveBeginPlay`)
  (bind (_direction _size) (`Timeline|SizeChage`)
    (:`Update`
      ;[1 1 1] Т.о. урон = 1 + 10*{0.5-0} = от 6 до 1
      (set `self.Damage` (+ (* 10 (+ (`self.Damage`) _size)) 1.0))
      (`self.SetActorScale3D` (`KismetMathLibrary.MakeVector` _size _size _size)))
    (:`Finished`
      (`KismetSystemLibrary.Delay` 0.0)
      (`self.K2_DestroyActor`))))

(fn `UserConstructionScript`
  (`parent.UserConstructionScript`))