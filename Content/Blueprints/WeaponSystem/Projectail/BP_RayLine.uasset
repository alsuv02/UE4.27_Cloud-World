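; BP_RayLine is a ray projectile actor that moves its Sphere along relative Z and damages actors it overlaps.
; A gate lets Tick stretch the Sphere's Z scale by a Speed-based step for about 0.3 seconds, then closes.
; A second gate applies one shrink step at that point, as Tick only reopens it without re-entering.
; The DecreasStop and ProjDestroy calls are never run.
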(event `MoveTick`
  ;[1 1 1] Comment
  (`SceneComponent.K2_SetRelativeLocation` (`self.Sphere`) (+ (`SceneComponent.RelativeLocation` (`self.Sphere`)) (`KismetMathLibrary.MakeVector` 0.0 0.0 (* (`self.Speed`) (`self.Delta Seconds`)))) false false))

(event `self.ReceiveBeginPlay`
  (`self.ExtantionBegin`))

(event `self.ReceiveTick`
  (params (DeltaSeconds :type "Float (single-precision)"))
  (set `self.Delta Seconds` DeltaSeconds)
  (`self.MoveTick`)
  (`self.ExtantionTick`)
  (`self.DecreaseTick`))

(event `ExtantionTick`
  (bind _sphere (`self.Sphere`))
  (bind _returnvalue (+ (`self.LifeTime`) (`self.Delta Seconds`)))
  ;[1 1 1] Comment
  (`/Engine/EditorBlueprintResources/StandardMacros.Gate` true :!label _label
    (:`Exit`
      (`SceneComponent.SetRelativeScale3D` _sphere (+ (`SceneComponent.RelativeScale3D` _sphere) (`KismetMathLibrary.MakeVector` 0.0 0.0 (/ (`self.Speed`) 3000.0))))
      (if (<= _returnvalue 0.3)
        (set `self.LifeTime` _returnvalue)
        (else
          (`self.DecreaseStart`)
          (`self.ExtantionStop`)
          (set `self.LifeTime` 0.0))))))

(event `ExtantionBegin`
  ;[1 1 1] Comment
  (goto _label :!via `Open`))

(event `ExtantionStop`
  ;[1 1 1] Comment
  (goto _label :!via `Close`))

(event `DecreaseStart`
  (bind _sphere (`self.Sphere`))
  (bind _returnvalue (+ (`self.LifeTime`) (`self.Delta Seconds`)))
  ;[1 1 1] Comment
  (`/Engine/EditorBlueprintResources/StandardMacros.Gate` true :!label _label_2
    (:`Exit`
      (`SceneComponent.SetRelativeScale3D` _sphere (- (`SceneComponent.RelativeScale3D` _sphere) (`KismetMathLibrary.MakeVector` 0.0 0.0 (/ (`self.Speed`) 3010.0))))
      (if (<= _returnvalue 1.0)
        (set `self.LifeTime` _returnvalue)))))

(event `DecreaseTick`
  ;[1 1 1] Comment
  (goto _label_2 :!via `Open`))

(event `DecreasStop`
  ;[1 1 1] Comment
  (goto _label_2 :!via `Close`))

(event `self.ReceiveActorBeginOverlap`
  (params (OtherActor :type "Actor Object Reference"))
  ;[1 1 1] Comment
  (`GameplayStatics.ApplyDamage` OtherActor (`self.Damage`) null self "/Script/Engine.DamageType"))

(fn `UserConstructionScript`)