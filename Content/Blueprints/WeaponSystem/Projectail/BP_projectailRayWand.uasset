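; Projectile for a ray wand weapon that damages what it hits and visually stretches as it flies.
; After BeginPlay opens a gate, each tick lengthens the Sphere component's Z scale in proportion to Speed, independent of delta time.
; When projectile movement stops, it applies damage to the hit actor, reports an AI damage sense event at the impact and calls ProjDestroy.
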(event `self.ReceiveBeginPlay`
  (bind _sphere (`self.Sphere`))
  (`parent.ReceiveBeginPlay`)
  (goto _label :!via `Open`))

(event `self.ReceiveTick`
  (params (DeltaSeconds :type "Float (single-precision)"))
  (bind _sphere (`self.Sphere`))
  (`parent.ReceiveTick` DeltaSeconds)
  (`/Engine/EditorBlueprintResources/StandardMacros.Gate` true :!label _label
    (:`Exit`
      (`SceneComponent.SetRelativeScale3D` _sphere (+ (`SceneComponent.RelativeScale3D` _sphere) (`KismetMathLibrary.MakeVector` 0.0 0.0 (/ (`self.Speed`) 10000.0)))))))

(event `self.ProjectileMovement.OnProjectileStop`
  (params (ImpactResult :type "HitResult Structure (by ref)"))
  (bind (_bblockinghit _binitialoverlap _time _distance _location _impactpoint _normal _impactnormal _physmat _hitactor) (`GameplayStatics.BreakHitResult` ImpactResult))
  (bind _damage (`self.Damage`))
  (`GameplayStatics.ApplyDamage` _hitactor _damage null self "/Script/Engine.DamageType")
  (`AISense_Damage.ReportDamageEvent` _hitactor self _damage _location (0.0 0.0 0.0) "Damage")
  (`self.ProjDestroy`))

(fn `UserConstructionScript`
  (`parent.UserConstructionScript`))