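; Blue Genie homing projectile that seeks out nearby enemies and self-destructs when it finds none.
; On spawn, a timeline animates the sphere's scale and destroys the actor when finished.
; A looping timer appears to drive SetTarget, which scans all enemy actors for the nearest within MinDistant (500 per the author's note).
; A found enemy becomes the projectile movement's homing target and stops the self-destruct timeline.
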(event `SelfDestraction`
  (bind (_direction _size) (`Timeline|SizeChamge` :!label _label)
    (:`Update`
      (`SceneComponent.SetWorldScale3D` (`self.Sphere`) (`KismetMathLibrary.MakeVector` _size _size _size)))
    (:`Finished`
      (set `self.IsDead` true)
      (`KismetSystemLibrary.Delay` 0.0)
      (`self.K2_DestroyActor`))))

(event `StopDestruction`
  (goto _label :!via `Stop`))

(event `self.ReceiveBeginPlay`
  (`parent.ReceiveBeginPlay`)
  (bind _asbp_main_character_cw (cast `/Game/Blueprints/BP_MainCharacterCW` (`GameplayStatics.GetPlayerCharacter` 0)))
  (set `self.As Main Character CW` _asbp_main_character_cw)
  (`KismetSystemLibrary.K2_SetTimerDelegate` (`|CreateDelegate` :!event `SetTarget`) 0.1 true)
  (`self.SelfDestraction`))

(event `SetTarget`
  (bind _nearestenemy (`self.NearestEnemy`))
  ;[1 1 1] Подгружаем врагов на уровне и смотрим, кто ближе всего (макс видимости -- 500 от снаряда)
  (if (not (`self.IsDead`))
    (bind _outactors (`GameplayStatics.GetAllActorsOfClass` "/Game/Blueprints/Enemy/BP_CharacterEnemyParent.BP_CharacterEnemyParent_C"))
    (for _array_element _outactors
      (bind _returnvalue (`KismetMathLibrary.VSize` (- (`self.K2_GetActorLocation` _array_element) (`self.K2_GetActorLocation`))))
      (if (< _returnvalue (`self.MinDistant`))
        (set `self.MinDistant` _returnvalue)
        (set `self.NearestEnemy` _array_element)))
    ;[1 1 1] Если кто-то отсеялся, нацеливаемся на него
    (`/Engine/EditorBlueprintResources/StandardMacros.IsValid` _nearestenemy
      (:`Is Valid`
        (if (not (`self.IsDead`))
          ;[1 1 1] Надеюсь комп выживет
          (set `ProjectileMovementComponent.HomingTargetComponent` (`self.GetComponentByClass` _nearestenemy "/Script/Engine.SceneComponent") (`self.ProjectileMovement`))
          (`self.StopDestruction`))))))

(fn `UserConstructionScript`
  (`parent.UserConstructionScript`))