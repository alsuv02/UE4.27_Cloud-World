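; Item-drop projectile in the weapon system that turns into a spawned actor where it lands.
; When its ProjectileMovement component stops, it spawns the ItemToSpawn class at the impact location, without destroying itself in this graph.
; The construction script sets the static mesh's world scale from the MyWorldScale variable.
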(event `self.ProjectileMovement.OnProjectileStop`
  (params (ImpactResult :type "HitResult Structure (by ref)"))
  (`|SpawnActorFromClass` (`self.ItemToSpawn`) (`KismetMathLibrary.MakeTransform` (`.Location` (`GameplayStatics.BreakHitResult` ImpactResult))) "Undefined" "OverrideRootScale" null null))

(fn `UserConstructionScript`
  (`parent.UserConstructionScript`)
  (`SceneComponent.SetWorldScale3D` (`self.StaticMesh`) (`self.MyWorldScale`)))