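; Wand fireball projectile that gains damage and swells in size the longer it flies.
; Tick increases Damage and sphere scale, while a looping timer either randomly bursts it, with odds rising as it grows, or enlarges the impact effect.
; On projectile stop, it applies radial falloff damage and destroys itself.
; A valid effect asset also triggers a scaled effect with a BP_EffectTimer for cleanup, plus direct hit damage.
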(event `self.ReceiveTick`
  (params (DeltaSeconds :type "Float (single-precision)"))
  (bind _sphere (`self.Sphere`))
  (`parent.ReceiveTick` DeltaSeconds)
  (set `self.Damage` (+ (* DeltaSeconds (`self.PlusDamagePerSeconds`)) (`self.Damage`)))
  (`SceneComponent.SetWorldScale3D` _sphere (+ (`KismetMathLibrary.MakeVector` DeltaSeconds DeltaSeconds DeltaSeconds) (`SceneComponent.K2_GetComponentScale` _sphere))))

(event `self.ReceiveBeginPlay`
  (`parent.ReceiveBeginPlay`)
  (`KismetSystemLibrary.K2_SetTimerDelegate` (delegate `chek for burst`) 0.2 true))

(event `chek for burst`
  (bind _relativescale3d_x (`KismetMathLibrary.BreakVector` (`SceneComponent.RelativeScale3D` (`self.Sphere`))))
  (bind _returnvalue (* _relativescale3d_x 20.0))
  (`KismetSystemLibrary.PrintString` (`KismetStringLibrary.Conv_DoubleToString` _returnvalue))
  (if (> (`KismetMathLibrary.RandomFloatInRange` _returnvalue 100.0) 95.0)
    (`ProjectileMovementComponent.StopSimulating` (`self.ProjectileMovement`) (`GameplayStatics.MakeHitResult` false false 0.0 0.0 (`self.K2_GetActorLocation`)))
    (`self.ProjDestroy`)
    (else
      (set `self.EffectScale` (* (`self.EffectScale`) 1.1)))))

(event `self.ProjectileMovement.OnProjectileStop`
  (params (ImpactResult :type "HitResult Structure (by ref)"))
  (bind (_bblockinghit _binitialoverlap _time _distance _location _impactpoint _normal _impactnormal _physmat _hitactor) (`GameplayStatics.BreakHitResult` ImpactResult))
  (bind _damage (`self.Damage`))
  (bind _effecttoplay (`self.EffectToPlay`))
  ;[1 1 1] Comment
  (`/Engine/EditorBlueprintResources/StandardMacros.IsValid` _effecttoplay
    (:`Is Valid`
      (bind _returnvalue (`NiagaraFunctionLibrary.SpawnSystemAtLocation` _effecttoplay (+ _location (`self.EffectOffset`)) (struct) (`self.EffectScale`)))
      (`|SpawnActorFromClass` "/Game/Blueprints/BP_EffectTimer.BP_EffectTimer_C" (`KismetMathLibrary.MakeTransform` (0.0 0.0 0.0)) "Undefined" "OverrideRootScale" null _returnvalue null)
      (`GameplayStatics.ApplyDamage` _hitactor _damage))
    (:`Is Not Valid`
      _))
  (`GameplayStatics.ApplyRadialDamageWithFalloff` :`BaseDamage` _damage :`MinimumDamage` 1.0 :`Origin` _location :`DamageInnerRadius` 150.0 :`DamageOuterRadius` 200.0 :`DamageFalloff` 1.0 :`DamageCauser` null :`InstigatedByController` null)
  (`self.ProjDestroy`))

(fn `UserConstructionScript`
  (`parent.UserConstructionScript`))