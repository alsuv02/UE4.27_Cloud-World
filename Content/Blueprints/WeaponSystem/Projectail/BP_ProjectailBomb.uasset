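; BP_ProjectailBomb is an explosive projectile in the weapon system that deals radial damage with falloff.
; It detonates when its ProjectileMovement stops, using the impact location, or when the Boom event supplies a location.
; Both triggers share one path that applies damage from the Damage, InnerRadius and OuterRadius variables, then briefly draws debug spheres for both radii.
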(event `Boom`
  (params (BoomLocation :type "Vector Structure"))
  (set `self.Origin` BoomLocation)
  (`GameplayStatics.ApplyRadialDamageWithFalloff` :`BaseDamage` (`self.Damage`) :`MinimumDamage` 1.0 :`Origin` (`self.Origin`) :`DamageInnerRadius` (`self.InnerRadius`) :`DamageOuterRadius` (`self.OuterRadius`) :`DamageFalloff` 1.0 :`DamageCauser` null :`InstigatedByController` null :!label _label)
  (`KismetSystemLibrary.DrawDebugSphere` (`self.Origin`) (`self.OuterRadius`) 12 (struct :`R` 1.0 :`G` 1.0 :`B` 1.0 :`A` 1.0) 0.2)
  (`KismetSystemLibrary.DrawDebugSphere` (`self.Origin`) (`self.InnerRadius`) 12 (struct :`R` 1.0 :`A` 1.0) 0.2))

(event `self.ProjectileMovement.OnProjectileStop`
  (params (ImpactResult :type "HitResult Structure (by ref)"))
  (set `self.Origin` (`.Location` (`GameplayStatics.BreakHitResult` ImpactResult)))
  (goto _label))

(fn `UserConstructionScript`
  (`parent.UserConstructionScript`))