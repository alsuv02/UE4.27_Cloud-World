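; Projectile variant for the weapon system whose scale and damage change over its lifetime.
; On BeginPlay it stores its starting damage and plays the SizeChage timeline, whose Size curve scales the actor and multiplies that damage, with a fixed minimum damage floor.
; When the timeline finishes, the actor destroys itself after a zero-length delay.
; Leftover debug prints and a damage override are disconnected and never run.
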(event `self.ReceiveBeginPlay`
  (`parent.ReceiveBeginPlay`)
  (set `self.StartDamage` (`self.Damage`))
  (bind (_direction _size) (`Timeline|SizeChage`)
    (:`Update`
      (bind _returnvalue (* (`self.StartDamage`) _size))
      (if (<= _returnvalue 4.0)
        (set `self.Damage` 4.0)
        (else
          (set `self.Damage` _returnvalue)))
      (bind _returnvalue_2 (/ _size 1.5))
      (`self.SetActorScale3D` (`KismetMathLibrary.MakeVector` _returnvalue_2 _returnvalue_2 _returnvalue_2)))
    (:`Finished`
      (`KismetSystemLibrary.Delay` 0.0)
      (`self.K2_DestroyActor`))))

(fn `UserConstructionScript`
  (`parent.UserConstructionScript`))