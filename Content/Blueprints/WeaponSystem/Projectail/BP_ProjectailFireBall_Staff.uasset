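; Fireball projectile for a staff weapon whose damage is tied to its changing size.
; On BeginPlay it runs the parent logic, then a SizeChange timeline sets uniform actor scale and recomputes Damage linearly from the same Size value.
; An author note indicates damage falls as the fireball shrinks.
; When the timeline finishes, the actor waits for a delay equal to the final Size value, then destroys itself.
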(event `self.ReceiveBeginPlay`
  (`parent.ReceiveBeginPlay`)
  (bind (_direction _size) (`Timeline|SizeChange`)
    (:`Update`
      ;[1 1 1] Т.о. урон = 1 + 10*{0.37-0} = от 4.7 до 1
      (set `self.Damage` (+ (* 10 _size) 1.0))
      (`self.SetActorScale3D` (`KismetMathLibrary.MakeVector` _size _size _size)))
    (:`Finished`
      (`KismetSystemLibrary.Delay` _size)
      (`self.K2_DestroyActor`))))

(fn `UserConstructionScript`
  (`parent.UserConstructionScript`))