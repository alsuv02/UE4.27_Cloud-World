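; BP_ProjectailBomb_Wand is a bomb projectile in the weapon system, named for the wand, that goes off when it bounces off an enemy.
; Its projectile movement bounce event casts the hit actor to BP_CharacterEnemyParent and ignores any other bounce.
; On an enemy hit it calls Boom at the impact location, then destroys itself after a zero-length delay.
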(event `self.ProjectileMovement.OnProjectileBounce`
  (params (ImpactResult :type "HitResult Structure (by ref)") (ImpactVelocity :type "Vector Structure (by ref)"))
  (bind (_bblockinghit _binitialoverlap _time _distance _location _impactpoint _normal _impactnormal _physmat _hitactor) (`GameplayStatics.BreakHitResult` ImpactResult))
  (cast `/Game/Blueprints/Enemy/BP_CharacterEnemyParent` _hitactor)
  (`self.Boom` _location)
  (`KismetSystemLibrary.Delay` 0.0)
  (`self.K2_DestroyActor`))

(fn `UserConstructionScript`
  (`parent.UserConstructionScript`))