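; Weapon child for the no-weapon state that casts single projectiles in front of the main character.
; Shoot passes a mana check, then switches on the current book: Ray and Genie spawn dedicated classes, others use the book's projectile map, with stats from per-weapon maps.
; Player velocity is added only when the book is BP_ChildNoBook.
; StandartSpell fires the NoneBook projectile without a mana check; a Ray line-trace block is unconnected.
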(event `self.ReceiveBeginPlay`
  (`parent.ReceiveBeginPlay`))

(event `self.Shoot`
  (bind _maincharacterref (`self.MainCharacterRef`))
  (bind _maincharacterref_2 (`self.MainCharacterRef`))
  (bind _maincharacterref_3 (`self.MainCharacterRef`))
  (bind _currentbookref (`/Game/Blueprints/BP_MainCharacterCW.CurrentBookRef` (`self.MainCharacterRef`)))
  (bind (_shootrotation_roll _shootrotation_pitch _shootrotation_yaw) (`KismetMathLibrary.BreakRotator` (`/Game/Blueprints/BP_MainCharacterCW.ShootRotation` _maincharacterref_2)))
  (bind _currentbookref_2 (`/Game/Blueprints/BP_MainCharacterCW.CurrentBookRef` (`self.MainCharacterRef`)))
  (bind (_shootrotation_roll_2 _shootrotation_pitch_2 _shootrotation_yaw_2) (`KismetMathLibrary.BreakRotator` (`/Game/Blueprints/BP_MainCharacterCW.ShootRotation` _maincharacterref)))
  (bind (_shootrotation_roll_3 _shootrotation_pitch_3 _shootrotation_yaw_3) (`KismetMathLibrary.BreakRotator` (`/Game/Blueprints/BP_MainCharacterCW.ShootRotation` _maincharacterref_3)))
  (bind _currentbookref_3 (`/Game/Blueprints/BP_MainCharacterCW.CurrentBookRef` (`self.MainCharacterRef`)))
  (bind _value (`BlueprintMapLibrary.Map_Find` (`/Game/Blueprints/WeaponSystem/BP_DadBook.SizeByWeapon` (`/Game/Blueprints/BP_MainCharacterCW.CurrentBookRef` (`self.MainCharacterRef`))) "NewEnumerator5"))
  (bind _value_2 (`BlueprintMapLibrary.Map_Find` (`/Game/Blueprints/WeaponSystem/BP_DadBook.SizeByWeapon` (`/Game/Blueprints/BP_MainCharacterCW.CurrentBookRef` (`self.MainCharacterRef`))) "NewEnumerator5"))
  (`parent.Shoot`)
  ;[1 1 1] Система манны
  (bind `_sucсess` (`self.ManaSpending` (`BlueprintMapLibrary.Map_Find` (`/Game/Blueprints/WeaponSystem/BP_DadBook.ManaPriceByWeapon` (`/Game/Blueprints/BP_MainCharacterCW.CurrentBookRef` (`self.MainCharacterRef`))) "NewEnumerator5")))
  (if `_sucсess`
    (switch `/Game/Blueprints/WeaponSystem/EN_Book` (`/Game/Blueprints/BP_MainCharacterCW.EN_BookCurrent` (`self.MainCharacterRef`))
      (:`NewEnumerator0`
        ;[1 1 1] Без оружия + остальные книги (одиночные снаряды)
        (bind _returnvalue (`|SpawnActorFromClass` "/Game/Blueprints/WeaponSystem/Projectail/BP_projectailRayNone.BP_projectailRayNone_C" (`KismetMathLibrary.MakeTransform` (+ (`self.K2_GetActorLocation` _maincharacterref_3) (* (`/Game/Blueprints/BP_MainCharacterCW.ShootVector` _maincharacterref_3) 120.0)) (`KismetMathLibrary.MakeRotator` _shootrotation_yaw_3 -90.0 _shootrotation_roll_3) (0.1 0.1 2.0)) "Undefined" "OverrideRootScale" null null))
        ;;[1 1 1] Comment
        (set `/Game/Blueprints/WeaponSystem/Projectail/BP_projectailParent.ManaPrice/sec` (`BlueprintMapLibrary.Map_Find` (`/Game/Blueprints/WeaponSystem/BP_DadBook.ManaPriceByWeapon` _currentbookref) "NewEnumerator5") _returnvalue)
        (set `/Game/Blueprints/WeaponSystem/Projectail/BP_projectailParent.Damage` (`BlueprintMapLibrary.Map_Find` (`/Game/Blueprints/WeaponSystem/BP_DadBook.DamageByWeapon` _currentbookref) "NewEnumerator5") _returnvalue)
        (cast `/Game/Blueprints/WeaponSystem/BookChild/BP_ChildNoBook` (`/Game/Blueprints/BP_MainCharacterCW.CurrentBookRef` (`self.MainCharacterRef`)))
        ;;;[0.1968 1 0] Parent
        (`self.AddPersVelocityToProj` _returnvalue))
      (:`NewEnumerator1`
        ;[1 1 1] Без оружия + остальные книги (одиночные снаряды)
        (bind _returnvalue_2 (`|SpawnActorFromClass` (`BlueprintMapLibrary.Map_Find` (`/Game/Blueprints/WeaponSystem/BP_DadBook.ProjectailByWeapon` (`/Game/Blueprints/BP_MainCharacterCW.CurrentBookRef` (`self.MainCharacterRef`))) "NewEnumerator5") (`KismetMathLibrary.MakeTransform` (+ (`self.K2_GetActorLocation` _maincharacterref) (* (`/Game/Blueprints/BP_MainCharacterCW.ShootVector` _maincharacterref) 120.0)) (`KismetMathLibrary.MakeRotator` _shootrotation_yaw_2 -90.0 _shootrotation_roll_2) (`KismetMathLibrary.MakeVector` _value_2 _value_2 _value_2)) "Undefined" "OverrideRootScale" null null :!label _label))
        (set `/Game/Blueprints/WeaponSystem/Projectail/BP_projectailParent.ManaPrice/sec` (`BlueprintMapLibrary.Map_Find` (`/Game/Blueprints/WeaponSystem/BP_DadBook.ManaPriceByWeapon` _currentbookref_3) "NewEnumerator5") _returnvalue_2)
        (set `/Game/Blueprints/WeaponSystem/Projectail/BP_projectailParent.Damage` (`BlueprintMapLibrary.Map_Find` (`/Game/Blueprints/WeaponSystem/BP_DadBook.DamageByWeapon` _currentbookref_3) "NewEnumerator5") _returnvalue_2)
        (cast `/Game/Blueprints/WeaponSystem/BookChild/BP_ChildNoBook` (`/Game/Blueprints/BP_MainCharacterCW.CurrentBookRef` (`self.MainCharacterRef`)))
        ;;[0.1968 1 0] Parent
        (`self.AddPersVelocityToProj` _returnvalue_2))
      (:`NewEnumerator2`
        ;[1 1 1] Без оружия + остальные книги (одиночные снаряды)
        (bind _returnvalue_3 (`|SpawnActorFromClass` "/Game/Blueprints/WeaponSystem/Projectail/BP_ProjectailGenieBlue.BP_ProjectailGenieBlue_C" (`KismetMathLibrary.MakeTransform` (+ (`self.K2_GetActorLocation` _maincharacterref_2) (* (`/Game/Blueprints/BP_MainCharacterCW.ShootVector` _maincharacterref_2) 120.0)) (`KismetMathLibrary.MakeRotator` _shootrotation_roll _shootrotation_pitch _shootrotation_yaw) (`KismetMathLibrary.MakeVector` _value _value _value)) "Undefined" "OverrideRootScale" null null))
        (set `/Game/Blueprints/WeaponSystem/Projectail/BP_projectailParent.ManaPrice/sec` (`BlueprintMapLibrary.Map_Find` (`/Game/Blueprints/WeaponSystem/BP_DadBook.ManaPriceByWeapon` _currentbookref_2) "NewEnumerator5") _returnvalue_3)
        (set `/Game/Blueprints/WeaponSystem/Projectail/BP_projectailParent.Damage` (`BlueprintMapLibrary.Map_Find` (`/Game/Blueprints/WeaponSystem/BP_DadBook.DamageByWeapon` _currentbookref_2) "NewEnumerator5") _returnvalue_3)
        (set `/Game/Blueprints/WeaponSystem/Projectail/BP_projectailParent.Size` (`BlueprintMapLibrary.Map_Find` (`/Game/Blueprints/WeaponSystem/BP_DadBook.SizeByWeapon` _currentbookref_2) "NewEnumerator5") _returnvalue_3)
        (cast `/Game/Blueprints/WeaponSystem/BookChild/BP_ChildNoBook` (`/Game/Blueprints/BP_MainCharacterCW.CurrentBookRef` (`self.MainCharacterRef`)))
        ;;[0.1968 1 0] Parent
        (`self.AddPersVelocityToProj` _returnvalue_3))
      (:`NewEnumerator3`
        (goto _label))
      (:`NewEnumerator4`
        (goto _label))
      (:`NewEnumerator5`
        (goto _label)))))

(event `StandartSpell`
  (bind _maincharacterref (`self.MainCharacterRef`))
  (bind (_shootrotation_roll _shootrotation_pitch _shootrotation_yaw) (`KismetMathLibrary.BreakRotator` (`/Game/Blueprints/BP_MainCharacterCW.ShootRotation` _maincharacterref)))
  (bind _nonebookref (`/Game/Blueprints/BP_MainCharacterCW.NoneBookRef` (`self.MainCharacterRef`)))
  (bind _value (`BlueprintMapLibrary.Map_Find` (`/Game/Blueprints/WeaponSystem/BP_DadBook.SizeByWeapon` (`/Game/Blueprints/BP_MainCharacterCW.NoneBookRef` (`self.MainCharacterRef`))) "NewEnumerator5"))
  ;[1 1 1] Без оружия + остальные книги (одиночные снаряды)
  (bind _returnvalue (`|SpawnActorFromClass` (`BlueprintMapLibrary.Map_Find` (`/Game/Blueprints/WeaponSystem/BP_DadBook.ProjectailByWeapon` (`/Game/Blueprints/BP_MainCharacterCW.NoneBookRef` (`self.MainCharacterRef`))) "NewEnumerator5") (`KismetMathLibrary.MakeTransform` (+ (`self.K2_GetActorLocation` _maincharacterref) (* (`/Game/Blueprints/BP_MainCharacterCW.ShootVector` _maincharacterref) 120.0)) (`KismetMathLibrary.MakeRotator` _shootrotation_yaw -90.0 _shootrotation_roll) (`KismetMathLibrary.MakeVector` _value _value _value)) "Undefined" "OverrideRootScale" null null))
  (set `/Game/Blueprints/WeaponSystem/Projectail/BP_projectailParent.ManaPrice/sec` (`BlueprintMapLibrary.Map_Find` (`/Game/Blueprints/WeaponSystem/BP_DadBook.ManaPriceByWeapon` _nonebookref) "NewEnumerator5") _returnvalue)
  (set `/Game/Blueprints/WeaponSystem/Projectail/BP_projectailParent.Damage` (`BlueprintMapLibrary.Map_Find` (`/Game/Blueprints/WeaponSystem/BP_DadBook.DamageByWeapon` _nonebookref) "NewEnumerator5") _returnvalue)
  ;;[0.1968 1 0] Parent
  (`self.AddPersVelocityToProj` _returnvalue))

(fn `UserConstructionScript`
  (`parent.UserConstructionScript`))