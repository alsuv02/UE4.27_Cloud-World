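; Wand weapon child that overrides Shoot to fire according to the character's current spell book.
; With the Ray book, it fires a mirrored fan of debug-drawn line traces around a centre ray, built from spring-arm mark vectors, and damages hit actors.
; Other books spawn one scaled projectile along the shoot direction, and only NoBook passes it to AddPersVelocityToProj.
; Damage, range and projectile class come from the book's per-weapon maps.
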(event `self.Shoot`
  (bind _maincharacterref (`self.MainCharacterRef`))
  (bind _maincharacterref_2 (`self.MainCharacterRef`))
  (bind _maincharacterref_3 (`self.MainCharacterRef`))
  (bind _springarmmark (`/Game/Blueprints/MainCharacterCW.SpringArmMark` _maincharacterref))
  (bind (_shootrotation_roll _shootrotation_pitch _shootrotation_yaw) (`KismetMathLibrary.BreakRotator` (`/Game/Blueprints/MainCharacterCW.ShootRotation` _maincharacterref_2)))
  (bind _springarmmark_2 (`/Game/Blueprints/MainCharacterCW.SpringArmMark` _maincharacterref_3))
  (bind _currentbookref (`/Game/Blueprints/MainCharacterCW.CurrentBookRef` _maincharacterref_2))
  (bind _projectailsize (`/Game/Blueprints/WeaponSystem/BP_DadBook.ProjectailSize` _currentbookref))
  (`parent.Shoot`)
  (cast `/Game/Blueprints/WeaponSystem/BookChild/BP_ChildRayBook` (`/Game/Blueprints/MainCharacterCW.CurrentBookRef` (`self.MainCharacterRef`))
    (:`then`
      ;[1 1 1] Без оружия + Рэй
      (for _index (range (+ (`self.RayNumber`) 1))
        (bind _output_get (set `self.Index` _index))
        (if (not (== _output_get 0))
          (bind (_outhit _returnvalue) (`KismetSystemLibrary.LineTraceSingle` :`Start` (`SceneComponent.K2_GetComponentLocation` (`/Game/Blueprints/MainCharacterCW.Cone` _maincharacterref)) :`End` (+ (* (`SceneComponent.GetRightVector` _springarmmark) (* (`self.Index`) (`self.RayAngle`))) (* (* (`SceneComponent.GetForwardVector` _springarmmark) -1.0) (`BlueprintMapLibrary.Map_Find` (`/Game/Blueprints/WeaponSystem/BP_DadBook.DistantByWeapon` (`/Game/Blueprints/MainCharacterCW.RayBookRef` _maincharacterref)) "NewEnumerator0"))) :`TraceChannel` "TraceTypeQuery1" :`DrawDebugType` "ForDuration" :`DrawTime` 0.2))
          (if _returnvalue
            ;;[1 1 1] причиняем урон
            (`GameplayStatics.ApplyDamage` (`.HitActor` (`GameplayStatics.BreakHitResult` _outhit)) (`BlueprintMapLibrary.Map_Find` (`/Game/Blueprints/WeaponSystem/BP_DadBook.DamageByWeapon` (`/Game/Blueprints/MainCharacterCW.RayBookRef` (`self.MainCharacterRef`))) "NewEnumerator0"))))
        (bind (_outhit_2 _returnvalue_2) (`KismetSystemLibrary.LineTraceSingle` :`Start` (`SceneComponent.K2_GetComponentLocation` (`/Game/Blueprints/MainCharacterCW.Cone` _maincharacterref_3)) :`End` (+ (* (`SceneComponent.GetRightVector` _springarmmark_2) (* (* (`self.Index`) -1) (`self.RayAngle`))) (* (* (`SceneComponent.GetForwardVector` _springarmmark_2) -1.0) (`BlueprintMapLibrary.Map_Find` (`/Game/Blueprints/WeaponSystem/BP_DadBook.DistantByWeapon` (`/Game/Blueprints/MainCharacterCW.RayBookRef` _maincharacterref_3)) "NewEnumerator0"))) :`TraceChannel` "TraceTypeQuery1" :`DrawDebugType` "ForDuration" :`DrawTime` 0.2))
        (if _returnvalue_2
          ;[1 1 1] причиняем урон
          (`GameplayStatics.ApplyDamage` (`.HitActor` (`GameplayStatics.BreakHitResult` _outhit_2)) (`BlueprintMapLibrary.Map_Find` (`/Game/Blueprints/WeaponSystem/BP_DadBook.DamageByWeapon` (`/Game/Blueprints/MainCharacterCW.RayBookRef` (`self.MainCharacterRef`))) "NewEnumerator0")))))
    (:`CastFailed`
      ;[1 1 1] Без оружия + остальные книги (одиночные снаряды)
      (bind _returnvalue_3 (`|SpawnActorFromClass` (`BlueprintMapLibrary.Map_Find` (`/Game/Blueprints/WeaponSystem/BP_DadBook.ProjectailByWeapon` _currentbookref) "NewEnumerator0") (`KismetMathLibrary.MakeTransform` (+ (`self.K2_GetActorLocation` _maincharacterref_2) (* (`/Game/Blueprints/MainCharacterCW.ShootVector` _maincharacterref_2) 120.0)) (`KismetMathLibrary.MakeRotator` _shootrotation_yaw -90.0 _shootrotation_roll) (`KismetMathLibrary.MakeVector` _projectailsize _projectailsize _projectailsize)) "Undefined" "OverrideRootScale" null null))
      (cast `/Game/Blueprints/WeaponSystem/BookChild/BP_ChildNoBook` (`/Game/Blueprints/MainCharacterCW.CurrentBookRef` (`self.MainCharacterRef`)))
      ;;[0.1968 1 0] Parent
      (`self.AddPersVelocityToProj` _returnvalue_3))))

(fn `UserConstructionScript`
  (`parent.UserConstructionScript`))