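; BP_ChildPistol is the pistol child weapon, which serves as a pickup and handles pistol shooting.
; Interact switches the character to the pistol, updates the weapon widget, destroys the item and shows the Pugach component.
; Shoot calls the parent, spends Shatters if enough remain, then branches on the current book.
; Fire deals radial falloff damage at the mouse position with debug spheres, while None spawns a projectile, both using the book's per-weapon maps.
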(event `/Game/Blueprints/I_Interactable.Interact`
  (bind _as_bp_main_character_cw (`self.As BP Main Character CW`))
  ;[1 1 1] Switch
  (`/Game/Blueprints/BP_MainCharacterCW.SwitchToPistol` _as_bp_main_character_cw)
  (`/Game/Blueprints/C_CloudWorld.CurrentWeaponWidgetUpdate` (`self.As C Cloud World`) (`GameplayStatics.GetObjectClass` self))
  (`self.DestroySelfItem`)
  (`SceneComponent.SetVisibility` (`/Game/Blueprints/BP_MainCharacterCW.pugach` _as_bp_main_character_cw) true false))

(event `self.Shoot`
  (bind _maincharacterref (`self.MainCharacterRef`))
  (bind _maincharacterref_2 (`self.MainCharacterRef`))
  (bind _maincharacterref_3 (`self.MainCharacterRef`))
  (bind _mouseposition (`/Game/Blueprints/BP_MainCharacterCW.MousePosition` _maincharacterref))
  (bind _firebookref (`/Game/Blueprints/BP_MainCharacterCW.FireBookRef` _maincharacterref))
  (bind (_shootrotation_roll _shootrotation_pitch _shootrotation_yaw) (`KismetMathLibrary.BreakRotator` (`/Game/Blueprints/BP_MainCharacterCW.ShootRotation` _maincharacterref_2)))
  (bind _currentbookref (`/Game/Blueprints/BP_MainCharacterCW.CurrentBookRef` _maincharacterref_2))
  (bind _returnvalue (- (`/Game/Blueprints/BP_MainCharacterCW.Shatters` _maincharacterref_3) 10))
  (bind _value (`BlueprintMapLibrary.Map_Find` (`/Game/Blueprints/WeaponSystem/BookChild/BP_ChildFireBook.OutterRadiusByWeapon` _firebookref) "NewEnumerator4"))
  (bind _value_2 (`BlueprintMapLibrary.Map_Find` (`/Game/Blueprints/WeaponSystem/BP_DadBook.SizeByWeapon` _currentbookref) "NewEnumerator4"))
  (bind _value_3 (`BlueprintMapLibrary.Map_Find` (`/Game/Blueprints/WeaponSystem/BookChild/BP_ChildFireBook.InnerRadiusByWeapon` _firebookref) "NewEnumerator4"))
  (`parent.Shoot`)
  (if (not (< _returnvalue 0))
    (set `/Game/Blueprints/BP_MainCharacterCW.Shatters` _returnvalue _maincharacterref_3)
    (switch `/Game/Blueprints/WeaponSystem/EN_Book` (`/Game/Blueprints/BP_MainCharacterCW.EN_BookCurrent` (`self.MainCharacterRef`))
      (:`NewEnumerator1`
        (`GameplayStatics.ApplyRadialDamageWithFalloff` :`Origin` _mouseposition :`DamageInnerRadius` _value_3 :`DamageOuterRadius` _value :`DamageCauser` null :`InstigatedByController` null)
        (`KismetSystemLibrary.DrawDebugSphere` _mouseposition _value_3 12 (struct :`R` 1.0 :`A` 1.0) 0.2)
        (`KismetSystemLibrary.DrawDebugSphere` _mouseposition _value 12 (struct :`R` 1.0 :`G` 1.0 :`B` 1.0 :`A` 1.0) 0.2))
      (:`NewEnumerator5`
        ;[1 1 1] Без оружия + остальные книги (одиночные снаряды)
        (bind _returnvalue_2 (`|SpawnActorFromClass` (`BlueprintMapLibrary.Map_Find` (`/Game/Blueprints/WeaponSystem/BP_DadBook.ProjectailByWeapon` _currentbookref) "NewEnumerator4") (`KismetMathLibrary.MakeTransform` (+ (`self.K2_GetActorLocation` _maincharacterref_2) (* (`/Game/Blueprints/BP_MainCharacterCW.ShootVector` _maincharacterref_2) 120.0)) (`KismetMathLibrary.MakeRotator` _shootrotation_yaw -90.0 _shootrotation_roll) (`KismetMathLibrary.MakeVector` _value_2 _value_2 _value_2)) "Undefined" "OverrideRootScale" null null))
        (cast `/Game/Blueprints/WeaponSystem/BookChild/BP_ChildNoBook` (`/Game/Blueprints/BP_MainCharacterCW.CurrentBookRef` (`self.MainCharacterRef`)))
        ;;[0.1968 1 0] Parent
        (`self.AddPersVelocityToProj` _returnvalue_2)))))

(fn `UserConstructionScript`
  (`parent.UserConstructionScript`))