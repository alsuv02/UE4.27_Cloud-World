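; BP_ChildRing is an interactable fetish item in the weapon system that gives the player the Ring.
; On Interact it switches the main character to the Ring, passes its own class to the Cloud World reference to update the current fetish widget, then calls DestroySelfItem.
; The character and Cloud World references are not set here, and the other events are disabled stubs.
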(event `/Game/Blueprints/I_Interactable.Interact`
  ;[1 1 1] Switch
  (`/Game/Blueprints/BP_MainCharacterCW.SwitchToRing` (`self.As BP Main Character CW`))
  (`/Game/Blueprints/C_CloudWorld.CurrentFetishWidgetUpdate` (`self.As C Cloud World`) (`GameplayStatics.GetObjectClass` self))
  (`self.DestroySelfItem`))

(fn `UserConstructionScript`
  (`parent.UserConstructionScript`))