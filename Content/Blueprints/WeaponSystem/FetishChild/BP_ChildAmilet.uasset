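; BP_ChildAmilet is the interactable amulet fetish pickup in the weapon system.
; Interact switches the main character to the amulet, passes this class to CCloudWorld to update the current fetish widget, and calls DestroySelfItem.
; It then makes the character's Amulet component visible without propagating to children.
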(event `/Game/Blueprints/I_Interactable.Interact`
  (bind _as_bp_main_character_cw (`self.As BP Main Character CW`))
  ;[1 1 1] Switch
  (`/Game/Blueprints/BP_MainCharacterCW.SwitchToAmulet` _as_bp_main_character_cw)
  (`/Game/Blueprints/C_CloudWorld.CurrentFetishWidgetUpdate` (`self.As C Cloud World`) (`GameplayStatics.GetObjectClass` self))
  (`self.DestroySelfItem`)
  (`SceneComponent.SetVisibility` (`/Game/Blueprints/BP_MainCharacterCW.amulet` _as_bp_main_character_cw) true false))

(fn `UserConstructionScript`
  (`parent.UserConstructionScript`))