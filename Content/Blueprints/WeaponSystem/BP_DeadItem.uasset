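; Interactable item actor in the weapon system that displays its name on a widget component and removes itself when interacted with.
; On BeginPlay it caches the WB_ItemWidget and fills in its name text from ItemName.
; ShowText sets the widget's hidden state from its SetHidden argument.
; Interact destroys the actor after a zero-length delay, with no inventory or pickup logic in this Blueprint.
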(event `self.ReceiveBeginPlay`
  (bind _aswb_item_widget (cast `/Game/Blueprints/Widgets/HUD/WB_ItemWidget` (`WidgetComponent.GetWidget` (`self.Widget`))))
  (set `self.WidgetRef` _aswb_item_widget)
  (`TextBlock.SetText` (`/Game/Blueprints/Widgets/HUD/WB_ItemWidget.ItemName` _aswb_item_widget) (`self.ItemName`)))

(event `/Game/Blueprints/I_Interactable.ShowText`
  (params (SetHidden :type Boolean) (MainCharRef :type "/Game/Blueprints/BP_MainCharacterCW Object Reference"))
  (`SceneComponent.SetHiddenInGame` (`self.Widget`) SetHidden false))

(event `/Game/Blueprints/I_Interactable.Interact`
  (`KismetSystemLibrary.Delay` 0.0)
  (`self.K2_DestroyActor`))

(fn `UserConstructionScript`)