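; BP_DadWeapon is a base weapon Blueprint for spell weapons, with empty Shoot and BurstShootStop events for children to fill in.
; On BeginPlay it caches player 0's BP_MainCharacterCW.
; ManaSpending deducts a child-supplied spell price from the character's mana and returns success, or prints a low-mana message and returns false.
; AddPersVelocityToProj adds the character's velocity to a projectile so it flies consistently with or against movement.
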(event `Shoot`
  ;[1 1 1] Comment
)

(event `self.ReceiveBeginPlay`
  (`parent.ReceiveBeginPlay`)
  (bind _asbp_main_character_cw (cast `/Game/Blueprints/BP_MainCharacterCW` (`GameplayStatics.GetPlayerCharacter` 0)))
  (set `self.MainCharacterRef` _asbp_main_character_cw))

(event `BurstShootStop`
  ;[1 1 1] Comment
)

(event `AddPersVelocityToProj`
  (params (PojRef :type "/Game/Blueprints/WeaponSystem/Projectail/BP_projectailParent Object Reference"))
  (bind _projectilemovement (`/Game/Blueprints/WeaponSystem/Projectail/BP_projectailParent.ProjectileMovement` PojRef))
  ;[1 1 1] Добавляем велосити пули велосити персонажа, чтобы пуля летела одинаково и по вектору движения, и против. (нужно вынести в парент как-нибудь)
  (set `MovementComponent.Velocity` (+ (`MovementComponent.Velocity` _projectilemovement) (`MovementComponent.Velocity` (`Pawn.GetMovementComponent` (`self.MainCharacterRef`)))) _projectilemovement))

(fn `ManaSpending`
  (params (SpellPrice :type "Float (double-precision)"))
  (returns (`Sucсess` :type Boolean))
  (bind _maincharacterref (`self.MainCharacterRef`))
  (bind _returnvalue (- (`/Game/Blueprints/BP_MainCharacterCW.CurrentMana` _maincharacterref) SpellPrice))
  ;[1 1 1] Проверяем, хватает ли манны, если хватает -- уменьшаем и возвращаем успех, если нет -- возвращаем неуспех
  ;;[1 1 1] Цена вытягивается в детях из ссылки на книгу.
  (if (< _returnvalue 0.0)
    (`KismetSystemLibrary.PrintString` "LowMana T_T")
    (return false)
    (else
      (set `/Game/Blueprints/BP_MainCharacterCW.CurrentMana` _returnvalue _maincharacterref)
      (return true))))

(fn `UserConstructionScript`
  (`parent.UserConstructionScript`))