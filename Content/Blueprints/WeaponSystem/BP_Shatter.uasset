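; BP_Shatter is a weapon-system actor that adds one to the main character's Shatters count, apparently as a pickup.
; Its ShowText event, when called with SetHidden false, increments Shatters on the supplied character reference, then destroys the actor after a zero-length delay.
; A call with SetHidden true does nothing, and the BeginPlay, overlap and Tick events are disabled stubs.
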(event `/Game/Blueprints/I_Interactable.ShowText`
  (params (SetHidden :type Boolean) (MainCharRef :type "/Game/Blueprints/BP_MainCharacterCW Object Reference"))
  (if (not SetHidden)
    (`/Engine/EditorBlueprintResources/StandardMacros.IncrementInt` (`/Game/Blueprints/BP_MainCharacterCW.Shatters` MainCharRef)
      (:`  `
        (`KismetSystemLibrary.Delay` 0.0)
        (`self.K2_DestroyActor`)))))

(fn `UserConstructionScript`
  (`parent.UserConstructionScript`))