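; BP_Spawner is a spawner actor that continuously creates СH_enemy_Child enemies at its own location.
; On BeginPlay it caches the player as MainCharacterCW and starts a looping one-second timer, presumably bound to SpawnEnemy.
; SpawnEnemy spawns an enemy, then clears the stored timer handle if the player is dead, so the death check follows each spawn.
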(event `self.ReceiveBeginPlay`
  ;[0 1 0.01344] Comment
  (bind _asmch_cloud_mag (cast `/Game/Blueprints/MainCharacterCW` (`GameplayStatics.GetPlayerCharacter` 0)))
  (set `self.As Top Down Character` _asmch_cloud_mag)
  (bind _returnvalue (`KismetSystemLibrary.K2_SetTimerDelegate` (`|CreateDelegate` :!event `Spawn Enemy`) 1.0 true))
  (set `self.Handler` _returnvalue))

(event `Spawn Enemy`
  (`|SpawnActorFromClass` "/Game/Blueprints/СH_enemy_Child.СH_enemy_Child_C" (`KismetMathLibrary.MakeTransform` (`self.K2_GetActorLocation`)) "Undefined" "OverrideRootScale" null null)
  (if (`/Game/Blueprints/MainCharacterCW.IsDead` (`self.As Top Down Character`))
    (`KismetSystemLibrary.K2_ClearAndInvalidateTimerHandle` (`self.Handler`))))

(fn `UserConstructionScript`)