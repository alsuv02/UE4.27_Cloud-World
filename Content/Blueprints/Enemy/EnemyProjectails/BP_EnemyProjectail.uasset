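; BP_EnemyProjectail is an enemy projectile that damages the actor it hits.
; When its ProjectileMovement stops, it applies its Damage to the hit actor unless the main character reference has IsRingSet on, then destroys itself.
; The damage path waits through a zero-length Delay before destruction, and BeginPlay and construction only call the parent.
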(event `self.ReceiveBeginPlay`
  (`parent.ReceiveBeginPlay`))

(event `self.ProjectileMovement.OnProjectileStop`
  (params (ImpactResult :type "HitResult Structure (by ref)"))
  (if (not (`/Game/Blueprints/BP_MainCharacterCW.IsRingSet?` (`self.As BP Main Character CW`)))
    (`GameplayStatics.ApplyDamage` (`.HitActor` (`GameplayStatics.BreakHitResult` ImpactResult)) (`self.Damage`))
    (`KismetSystemLibrary.Delay` 0.0))
  (`self.K2_DestroyActor`))

(fn `UserConstructionScript`
  (`parent.UserConstructionScript`))