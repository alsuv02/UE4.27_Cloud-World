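; Ally character Blueprint that reuses enemy types such as AIC_Enemy and the enemy health bar widget, with nearly all of its logic disconnected.
; BeginPlay, AnyDamage, Death, SetDethCollision and DropShatters are empty events.
; Their apparent bodies (health bar binding, damage, death cleanup, radial shatter spawning) are orphaned and never run.
; Only the construction script works, setting health to max, assigning CurrentMana to itself and caching the AI controller.
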(event `self.ReceiveBeginPlay`)

(event `self.ReceiveAnyDamage`
  (params (Damage :type "Float (single-precision)") (DamageType :type "DamageType Object Reference") (InstigatedBy :type "Controller Object Reference") (DamageCauser :type "Actor Object Reference"))
  ;[1 1 1] Пешка получает урон
)

(event `Death`
  ;[0 0 0] Comment
)

(event `SetDethCollision`
  ;[0 0 0] Comment
)

(event `DropShatters`
  ;[0 0 0] Comment
  ;;[1 1 1] SpawnShatters hehe boy
)

(fn `UserConstructionScript`
  (set `self.CurrentHealth` (`self.MaxHealth`))
  (set `self.CurrentMana` (`self.CurrentMana`))
  (bind _asaic_enemy (cast `/Game/Blueprints/Enemy/AI/AIC_Enemy` (`self.GetController`)))
  (set `self.As AIC Enemy` _asaic_enemy))