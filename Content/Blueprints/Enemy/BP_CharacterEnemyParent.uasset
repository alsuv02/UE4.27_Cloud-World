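; Base enemy character that tracks health and shows a health bar when it takes damage.
; BeginPlay passes the character to its HUD_EnemyHealthBar widget, which AnyDamage makes visible before subtracting health or calling Death on lethal damage.
; Death destroys the actor after a brief delay.
; The construction script fills health to maximum, assigns current mana to itself and caches the AIC_Enemy controller.
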(event `self.ReceiveBeginPlay`
  (bind _ashud_enemy_health_bar (cast `/Game/Blueprints/Enemy/HUD_EnemyHealthBar` (`WidgetComponent.GetUserWidgetObject` (`self.HealthBar`))))
  (bind _output_get (set `self.As HUD Enemy Health Bar` _ashud_enemy_health_bar))
  (set `/Game/Blueprints/Enemy/HUD_EnemyHealthBar.EnemyCharacterRef` self _output_get))

(event `self.ReceiveAnyDamage`
  (params (Damage :type "Float (single-precision)") (DamageType :type "DamageType Object Reference") (InstigatedBy :type "Controller Object Reference") (DamageCauser :type "Actor Object Reference"))
  (bind _returnvalue (- (`self.CurrentHealth`) Damage))
  ;[1 1 1] Пешка получает урон
  (`Widget.SetVisibility` (`/Game/Blueprints/Enemy/HUD_EnemyHealthBar.ProgressBar_28` (`self.As HUD Enemy Health Bar`)) "Visible")
  (if (<= _returnvalue 0.0)
    (`self.Death`)
    (else
      (set `self.CurrentHealth` _returnvalue))))

(event `Death`
  ;[0 0 0] Comment
  (`KismetSystemLibrary.Delay` 0.01)
  (`self.K2_DestroyActor`))

(fn `UserConstructionScript`
  (set `self.CurrentHealth` (`self.MaxHealth`))
  (set `self.CurrentMana` (`self.CurrentMana`))
  (bind _asaic_enemy (cast `/Game/Blueprints/Enemy/AI/AIC_Enemy` (`self.GetController`)))
  (set `self.As AIC Enemy` _asaic_enemy))