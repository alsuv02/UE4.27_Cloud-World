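; Arena encounter controller that locks the player in on their first entry into its trigger box and spawns a configured set of enemies.
; Entry raises chest fences, shows gates, and spawns enemies by type at offsets from the actor, each holding a controller reference.
; Removal requests prune the enemy list; after a retriggerable delay, no valid enemies left means notifying BP_BossGate, destroying gates and lowering fences.
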(event `self.TriggerBox.OnComponentBeginOverlap`
  (params (OverlappedComponent :type "PrimitiveComponent Object Reference") (OtherActor :type "Actor Object Reference") (OtherComp :type "PrimitiveComponent Object Reference") (OtherBodyIndex :type Integer) (bFromSweep :type Boolean) (SweepResult :type "HitResult Structure (by ref)"))
  (cast `/Game/Blueprints/BP_MainCharacterCW` OtherActor)
  (if (`self.IsFirstVisit?`)
    (set `self.IsFirstVisit?` false)
    (`KismetSystemLibrary.Delay` 0.1)
    (`self.UpChestGate`)
    ;[0.1146 1 0] SpawnEnemy
    (for (_array_element _array_index) (`self.EnemyTypeToSpawn`)
      (switch `/Game/Blueprints/Enemy/EN_Enemy` _array_element
        (:`NewEnumerator0`
          _)
        (:`NewEnumerator1`
          _)
        (:`NewEnumerator2`
          _)
        (:`NewEnumerator3`
          _))
      (bind _returnvalue (`|SpawnActorFromClass` (select `/Game/Blueprints/Enemy/EN_Enemy` _array_element :`NewEnumerator0` "/Game/Blueprints/Enemy/BP_ArcherCharacterEnemy.BP_ArcherCharacterEnemy_C" :`NewEnumerator1` "/Game/Blueprints/Enemy/BP_MeleeCharacterEnemy.BP_MeleeCharacterEnemy_C" :`NewEnumerator2` "/Game/Blueprints/Enemy/BP_EnchantressCharacterEnemy.BP_EnchantressCharacterEnemy_C" :`NewEnumerator3` "/Game/Blueprints/Enemy/BP_KamikazeCharacterEnemy.BP_KamikazeCharacterEnemy_C" :!type "Actor Class Reference") (`KismetMathLibrary.MakeTransform` (+ (`self.K2_GetActorLocation`) (`|GetArrayItem` (`self.EnemySpawnPoints`) _array_index))) "Undefined" "OverrideRootScale" null null))
      (bind _asbp_character_enemy_parent (cast `/Game/Blueprints/Enemy/BP_CharacterEnemyParent` _returnvalue :!pure true))
      (set `/Game/Blueprints/Enemy/BP_CharacterEnemyParent.ArenaControllerRef` self _asbp_character_enemy_parent)
      (`KismetArrayLibrary.Array_Add` (`self.EnemyArrey`) _asbp_character_enemy_parent))))

(event `RemoveEnemyFromSet`
  (params (EnemyRef :type "/Game/Blueprints/Enemy/BP_CharacterEnemyParent Object Reference"))
  (bind _enemyarrey (`self.EnemyArrey`))
  ;[0 0 0] Comment
  (`KismetArrayLibrary.Array_RemoveItem` _enemyarrey EnemyRef)
  (`KismetSystemLibrary.RetriggerableDelay` 0.1)
  ;;[1 1 1] Comment
  (for _array_element _enemyarrey
    (`/Engine/EditorBlueprintResources/StandardMacros.IsValid` _array_element
      (:`Is Valid`
        (`/Engine/EditorBlueprintResources/StandardMacros.IncrementInt` (`self.EmptyArreyCheckIndex`)))))
  (if (== (`self.EmptyArreyCheckIndex`) 0)
    (`self.RemoveGates`)
    (else
      (set `self.EmptyArreyCheckIndex` 0))))

(event `UpChestGate`
  ;[1 1 1] Comment
  (for _array_element (`self.ChestArrayRef`)
    (`/Game/Blueprints/environment/BP_Chest.SetFence` _array_element true))
  (for _array_element_2 (`self.GatesArrayRef`)
    (`/Game/Blueprints/environment/BP_Gate.SetVisible` _array_element_2 true)))

(event `RemoveGates`
  ;[0 0 0] Comment
  (bind _returnvalue (`GameplayStatics.GetActorOfClass` "/Game/Blueprints/environment/BP_BossGate.BP_BossGate_C"))
  (`/Game/Blueprints/environment/BP_BossGate.BossReadyCheck` _returnvalue)
  (for _array_element (`self.GatesArrayRef`)
    (`self.K2_DestroyActor` _array_element))
  (`self.DownChestGate`))

(event `DownChestGate`
  ;[1 1 1] Comment
  (for _array_element (`self.ChestArrayRef`)
    (`/Game/Blueprints/environment/BP_Chest.SetFence` _array_element false))
  (for _array_element_2 (`self.GatesArrayRef`)
    (`/Game/Blueprints/environment/BP_Gate.SetVisible` _array_element_2 false)))

(fn `UserConstructionScript`
  (`SceneComponent.SetWorldScale3D` (`self.TriggerBox`) (`self.TriggerBoxScale`)))