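; Boss arena controller that locks the player in on first trigger overlap and runs enemy waves.
; Randomize picks random enemy types; SpawnWave runs inside that loop, re-spawning the growing, never-cleared array at preset offsets.
; Spawned enemies reference the controller; RemoveEnemyfromSet uses a retriggerable delay before checking for survivors and advancing waves.
; After the last wave it calls BP_BossGate's BossReadyCheck, destroys the gates and calls Victory inside the gate-hiding loop.
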(event `self.ReceiveBeginPlay`
  ;[1 1 1] Comment
  (bind _asc_cloud_world (cast `/Game/Blueprints/C_CloudWorld` (`GameplayStatics.GetPlayerController` 0)))
  (set `self.As C Cloud World` _asc_cloud_world))

(event `self.TriggerBox.OnComponentBeginOverlap`
  (params (OverlappedComponent :type "PrimitiveComponent Object Reference") (OtherActor :type "Actor Object Reference") (OtherComp :type "PrimitiveComponent Object Reference") (OtherBodyIndex :type Integer) (bFromSweep :type Boolean) (SweepResult :type "HitResult Structure (by ref)"))
  ;[1 1 1] Comment
  (cast `/Game/Blueprints/BP_MainCharacterCW` OtherActor)
  (if (`self.IsFirstVisit?`)
    (set `self.IsFirstVisit?` false)
    (`KismetSystemLibrary.Delay` 0.1)
    (`self.UpChestGate`)
    (`self.Randomize`)))

(event `Randomize`
  ;[1 1 1] Готовим волну к десанту
  (for _ (range (`self.EnemyAmount`))
    (bind _output_get (set `self.EnemyType` (select `int` (`KismetMathLibrary.RandomIntegerInRange` 0 3) :`0` "NewEnumerator0" :`1` "NewEnumerator1" :`2` "NewEnumerator2" :`3` "NewEnumerator3" :!type "/Game/Blueprints/Enemy/EN_Enemy Enum")))
    (`KismetArrayLibrary.Array_Add` (`self.ArrayEnemyToSpawn`) (select `/Game/Blueprints/Enemy/EN_Enemy` _output_get :`NewEnumerator0` (`self.Archer`) :`NewEnumerator1` (`self.Melee`) :`NewEnumerator2` (`self.Enchantress`) :`NewEnumerator3` (`self.Kamikaze`)))
    (`self.SpawnWave`)))

(event `self.UpChestGate`
  ;[1 1 1] Comment
  (for _array_element (`self.GatesArrayRef`)
    (`/Game/Blueprints/environment/BP_Gate.SetVisible` _array_element true)))

(event `SpawnWave`
  ;[0.1146 1 0] SpawnEnemy
  (for (_array_element _array_index) (`self.ArrayEnemyToSpawn`)
    (bind _returnvalue (`|SpawnActorFromClass` _array_element (`KismetMathLibrary.MakeTransform` (+ (`self.K2_GetActorLocation`) (`|GetArrayItem` (`self.EnemySpawnPoints`) _array_index))) "Undefined" "OverrideRootScale" null null))
    (set `/Game/Blueprints/Enemy/BP_CharacterEnemyParent.ArenaControllerRef` self _returnvalue)
    (`KismetArrayLibrary.Array_Add` (`self.EnemyArrey`) _returnvalue)))

(event `self.DownChestGate`
  ;[1 1 1] Comment
  (for _array_element (`self.GatesArrayRef`)
    (`/Game/Blueprints/environment/BP_Gate.SetVisible` _array_element false)
    (`/Game/Blueprints/C_CloudWorld.Victory` (`self.As C Cloud World`))))

(event `self.RemoveEnemyFromSet`
  (params (EnemyRef :type "/Game/Blueprints/Enemy/BP_CharacterEnemyParent Object Reference"))
  (bind _enemyarrey (`self.EnemyArrey`))
  ;[0 0 0] Comment
  (`KismetArrayLibrary.Array_RemoveItem` _enemyarrey EnemyRef)
  (`KismetSystemLibrary.RetriggerableDelay` 0.1)
  ;;[1 1 1] Comment
  (for _array_element _enemyarrey
    (`/Engine/EditorBlueprintResources/StandardMacros.IsValid` _array_element
      (:`Is Valid`
        (`/Engine/EditorBlueprintResources/StandardMacros.IncrementInt` (`self.EmptyArreyCheckIndex`)))))
  (if (== (`self.EmptyArreyCheckIndex`) 0)
    (`self.IsLastWave?`)
    (else
      (set `self.EmptyArreyCheckIndex` 0))))

(event `IsLastWave?`
  ;[0 0 0] Comment
  ;;[1 1 1] Comment
  (if (>= (`self.CurrentWave`) (`self.WaveAmount`))
    (`self.RemoveGates`)
    (else
      (`/Engine/EditorBlueprintResources/StandardMacros.IncrementInt` (`self.CurrentWave`)
        (:`  `
          (`self.Randomize`))))))

(event `self.RemoveGates`
  ;[0 0 0] Comment
  ;;[1 1 1] Comment
  (bind _returnvalue (`GameplayStatics.GetActorOfClass` "/Game/Blueprints/environment/BP_BossGate.BP_BossGate_C"))
  (`/Game/Blueprints/environment/BP_BossGate.BossReadyCheck` _returnvalue)
  (for _array_element (`self.GatesArrayRef`)
    (`self.K2_DestroyActor` _array_element))
  (`self.DownChestGate`))

(fn `UserConstructionScript`
  (`parent.UserConstructionScript`))