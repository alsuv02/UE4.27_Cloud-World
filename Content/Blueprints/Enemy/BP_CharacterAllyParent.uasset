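; BP_CharacterAllyParent is the parent Blueprint for temporary ally characters, with a health bar widget and a limited lifespan.
; BeginPlay links the widget to the ally and caches the player character, while the construction script initializes health and caches an AIC_Enemy controller.
; Tick drains health in proportion to MaxHealth over the lifetime.
; At zero, Death decrements the pistol's GenieCounter and destroys the actor after a short delay.
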(event `self.ReceiveBeginPlay`
  ;[1 1 1] Comment
  (bind _ashud_ally_health_bar (cast `/Game/Blueprints/Widgets/PopUp/HUD_AllyHealthBar` (`WidgetComponent.GetUserWidgetObject` (`self.HealthBar`))))
  (bind _output_get (set `self.As HUD Ally Health Bar` _ashud_ally_health_bar))
  (set `/Game/Blueprints/Widgets/PopUp/HUD_AllyHealthBar.AllyCharacterRef` self _output_get)
  (bind _asbp_main_character_cw (cast `/Game/Blueprints/BP_MainCharacterCW` (`GameplayStatics.GetPlayerCharacter` 0)))
  (set `self.As BP Main Character CW` _asbp_main_character_cw)
  (`Widget.SetVisibility` (`/Game/Blueprints/Widgets/PopUp/HUD_AllyHealthBar.ProgressBar_28` (`self.As HUD Ally Health Bar`)) "Visible"))

(event `self.ReceiveTick`
  (params (DeltaSeconds :type "Float (single-precision)"))
  (bind _returnvalue (- (`self.CurrentHealth`) (/ (* (`self.MaxHealth`) DeltaSeconds) (`self.AllyLifeTime/sec`))))
  ;[1 1 1] Счётчик жизни
  (if (<= _returnvalue 0.0)
    (set `self.CurrentHealth` 0.0)
    (`self.Death`)
    (else
      (set `self.CurrentHealth` _returnvalue))))

(event `Death`
  (bind _pistolref (`self.PistolRef`))
  ;[0 0 0] Comment
  (set `self.IsDead` true)
  (set `/Game/Blueprints/WeaponSystem/WeaponChild/BP_ChildPistol.GenieCounter` (- (`/Game/Blueprints/WeaponSystem/WeaponChild/BP_ChildPistol.GenieCounter` _pistolref) 1) _pistolref)
  (`KismetSystemLibrary.Delay` 0.01)
  (`self.K2_DestroyActor`))

(fn `UserConstructionScript`
  (set `self.CurrentHealth` (`self.MaxHealth`))
  (set `self.CurrentMana` (`self.CurrentMana`))
  (bind _asaic_enemy (cast `/Game/Blueprints/Enemy/AI/AIC_Enemy` (`self.GetController`)))
  (set `self.As AIC Enemy` _asaic_enemy))