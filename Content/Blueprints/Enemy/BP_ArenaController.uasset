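; BP_ArenaController runs a one-time combat arena that locks behind gates when the main character enters its scalable trigger box.
; After a short delay, it spawns gates at actor-offset points and enemies by type at index-matched spawn points, giving each enemy a controller reference.
; RemoveEnemyFromSet drops an enemy, recounts valid ones after a retriggerable delay, and destroys the gates when none remain.
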(event `self.TriggerBox.OnComponentBeginOverlap`
  (params (OverlappedComponent :type "PrimitiveComponent Object Reference") (OtherActor :type "Actor Object Reference") (OtherComp :type "PrimitiveComponent Object Reference") (OtherBodyIndex :type Integer) (bFromSweep :type Boolean) (SweepResult :type "HitResult Structure (by ref)"))
  (cast `/Game/Blueprints/BP_MainCharacterCW` OtherActor)
  (if (`self.IsFirstVisit?`)
    (set `self.IsFirstVisit?` false)
    (`KismetSystemLibrary.Delay` 0.2)
    ;[0.1384 1 0] Спавним преграду
    (for _array_element (`self.GateSpawnPoints`)
      (bind _returnvalue (`|SpawnActorFromClass` "/Game/Blueprints/BP_Gate.BP_Gate_C" (`KismetMathLibrary.MakeTransform` (+ _array_element (`self.K2_GetActorLocation`))) "AlwaysSpawn" "OverrideRootScale" null null))
      (`KismetArrayLibrary.Array_Add` (`self.GatesArray`) _returnvalue))
    ;[0.1146 1 0] SpawnEnemy
    (for (_array_element_2 _array_index) (`self.EnemyTypeToSpawn`)
      (switch `/Game/Blueprints/Enemy/EN_Enemy` _array_element_2
        (:`NewEnumerator0`
          _)
        (:`NewEnumerator1`
          _)
        (:`NewEnumerator2`
          _)
        (:`NewEnumerator3`
          _))
      (bind _returnvalue_2 (`|SpawnActorFromClass` (select `/Game/Blueprints/Enemy/EN_Enemy` _array_element_2 :`NewEnumerator0` "/Game/Blueprints/Enemy/BP_ArcherCharacterEnemy.BP_ArcherCharacterEnemy_C" :`NewEnumerator1` "/Game/Blueprints/Enemy/BP_MeleeCharacterEnemy.BP_MeleeCharacterEnemy_C" :`NewEnumerator2` "/Game/Blueprints/Enemy/BP_EnchantressCharacterEnemy.BP_EnchantressCharacterEnemy_C" :`NewEnumerator3` "/Game/Blueprints/Enemy/BP_KamikazeCharacterEnemy.BP_KamikazeCharacterEnemy_C" :!type "Actor Class Reference") (`KismetMathLibrary.MakeTransform` (`|GetArrayItem` (`self.EnemySpawnPoints`) _array_index)) "Undefined" "OverrideRootScale" null null))
      (bind _asbp_character_enemy_parent (cast `/Game/Blueprints/Enemy/BP_CharacterEnemyParent` _returnvalue_2 :!pure true))
      (set `/Game/Blueprints/Enemy/BP_CharacterEnemyParent.ArenaControllerRef` self _asbp_character_enemy_parent)
      (`KismetArrayLibrary.Array_Add` (`self.EnemyArrey`) _asbp_character_enemy_parent))))

(event `self.ReceiveBeginPlay`
  ;[1 0 0.793] Comment
)

(event `ReCheck`
  ;[1 0 0.793] Comment
)

(event `RemoveEnemyFromSet`
  (params (EnemyRef :type "/Game/Blueprints/Enemy/BP_CharacterEnemyParent Object Reference"))
  (bind _enemyarrey (`self.EnemyArrey`))
  ;[0 0 0] Comment
  (`KismetArrayLibrary.Array_RemoveItem` _enemyarrey EnemyRef)
  (`KismetSystemLibrary.RetriggerableDelay` 0.1)
  ;;[1 1 1] Comment
  (for _array_element _enemyarrey
    (`/Engine/EditorBlueprintResources/StandardMacros.IsValid` _array_element
      (:`Is Valid`
        (`/Engine/EditorBlueprintResources/StandardMacros.IncrementInt` (`self.EmptyArreyCheckIndex`)))))
  (if (== (`self.EmptyArreyCheckIndex`) 0)
    (`self.RemoveGates`)
    (else
      (set `self.EmptyArreyCheckIndex` 0))))

(event `RemoveGates`
  ;[0 0 0] Comment
  (for _array_element (`self.GatesArray`)
    (`self.K2_DestroyActor` _array_element)
    (`KismetArrayLibrary.Array_RemoveItem` (`self.GatesArray`) _array_element)))

(fn `UserConstructionScript`
  (`SceneComponent.SetWorldScale3D` (`self.TriggerBox`) (`self.TriggerBoxScale`)))