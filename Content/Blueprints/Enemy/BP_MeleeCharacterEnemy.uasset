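; BP_MeleeCharacterEnemy is a melee enemy character that builds on a parent class.
; On BeginPlay it runs the parent logic, then adds its Helmet and Sword to the ComponentToBroke array, noted as components to remove on death.
; The removal itself is not in these graphs, and the construction script only calls the parent.
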(event `self.ReceiveBeginPlay`
  (bind _componenttobroke (`self.ComponentToBroke`))
  (`parent.ReceiveBeginPlay`)
  ;[1 1 1] Устанавливаем компоненты, которые нужно удалить при смерти
  (`KismetArrayLibrary.Array_Add` _componenttobroke (`self.helmet`))
  (`KismetArrayLibrary.Array_Add` _componenttobroke (`self.sword`)))

(fn `UserConstructionScript`
  (`parent.UserConstructionScript`))