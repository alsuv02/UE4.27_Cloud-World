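; BP_BossGate is a gate that blocks the boss until the other arena rooms have been visited.
; BossReadyCheck counts BP_ArenaControllers still flagged IsFirstVisit, minus one, then either stores the remainder or hides the gate and ignores its collision.
; BeginPlay runs the check and writes a Russian "fights left" remaining/total label to the WB_ItemWidget.
; ShowText toggles that widget only while the gate is visible.
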(event `BossReadyCheck`
  ;[1 1 1] Comment
  (bind _outactors (`GameplayStatics.GetAllActorsOfClass` "/Game/Blueprints/Enemy/ArenaControllers/BP_ArenaController.BP_ArenaController_C"))
  (set `self.RoomsAll` (- (`KismetArrayLibrary.Array_Length` _outactors) 1))
  (for _array_element _outactors
    (if (`/Game/Blueprints/Enemy/ArenaControllers/BP_ArenaController.IsFirstVisit?` _array_element)
      (`/Engine/EditorBlueprintResources/StandardMacros.IncrementInt` (`self.Counter`))))
  ;[1 1 1] Comment
  (set `self.Counter` (- (`self.Counter`) 1))
  (if (> (`self.Counter`) 0)
    (set `self.RoomsToClearLeft` (`self.Counter`))
    (set `self.Counter` 0)
    (else
      (`SceneComponent.SetVisibility` (`self.gates`) false false)
      (`PrimitiveComponent.SetCollisionResponseToAllChannels` (`self.gates`) "ECR_Ignore"))))

(event `/Game/Blueprints/I_Interactable.ShowText`
  (params (SetHidden :type Boolean) (MainCharRef :type "/Game/Blueprints/BP_MainCharacterCW Object Reference"))
  ;[1 1 1] Comment
  (if (`SceneComponent.IsVisible` (`self.gates`))
    (`SceneComponent.SetHiddenInGame` (`self.Widget`) SetHidden false)))

(event `self.ReceiveBeginPlay`
  ;[1 1 1] Comment
  (`self.BossReadyCheck`)
  (bind _output_get (set `self.As WB Item Widget` (cast `/Game/Blueprints/Widgets/PopUp/WB_ItemWidget` (`WidgetComponent.GetWidget` (`self.Widget`)) :!pure true)))
  (`TextBlock.SetText` (`/Game/Blueprints/Widgets/PopUp/WB_ItemWidget.line1` _output_get) "Боёв осталось")
  (`TextBlock.SetText` (`/Game/Blueprints/Widgets/PopUp/WB_ItemWidget.Line2` _output_get) (`KismetTextLibrary.Conv_StringToText` (`KismetStringLibrary.Concat_StrStr` (`KismetStringLibrary.Conv_IntToString` (`self.RoomsToClearLeft`)) "/" (`KismetStringLibrary.Conv_IntToString` (`self.RoomsAll`))))))

(fn `UserConstructionScript`)