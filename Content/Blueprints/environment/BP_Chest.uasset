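; Loot chest actor with a name widget that drops a random item and a burst of shatters on a one-time interaction.
; Interact hides the chest as a stopgap, then asks the C_CloudWorld player controller for an item type and maps it to a projectile class.
; Drops and shatters spawn above the chest and launch with randomized angles and speeds.
; SetFence toggles visibility and collision of four fence components while IsClose is true.
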(event `SetFence`
  (params (SetUp :type Boolean))
  (if (`self.IsClose?`)
    (`self.SetFenceMacros` SetUp)))

(event `self.ReceiveBeginPlay`
  ;[0.09245 1 0] Comment
  (bind _asc_cloud_world (cast `/Game/Blueprints/C_CloudWorld` (`GameplayStatics.GetPlayerController` 0)))
  (set `self.As C Cloud World` _asc_cloud_world)
  (`self.SetFence` false)
  (bind _aswb_item_widget (cast `/Game/Blueprints/Widgets/PopUp/WB_ItemWidget` (`WidgetComponent.GetWidget` (`self.Widget`))))
  (set `self.WidgetRef` _aswb_item_widget)
  (`TextBlock.SetText` (`/Game/Blueprints/Widgets/PopUp/WB_ItemWidget.line1` _aswb_item_widget) (`self.ItemName`)))

(event `/Game/Blueprints/I_Interactable.ShowText`
  (params (SetHidden :type Boolean) (MainCharRef :type "/Game/Blueprints/BP_MainCharacterCW Object Reference"))
  ;[1 1 1] Comment
  (`SceneComponent.SetHiddenInGame` (`self.Widget`) SetHidden false))

(event `/Game/Blueprints/I_Interactable.Interact`
  ;[1 1 1] Comment
  (if (`self.IsClose?`)
    (set `self.IsClose?` false)
    ;;[1 0.4162 0] Временная мера, пока актор просто прячется
    (`self.SetActorHiddenInGame` true)
    (`self.SetActorEnableCollision` false)
    (`self.GenerateItemToDrop`)))

(event `GenerateItemToDrop`
  ;[1 1 1] Comment
  (set `self.ShattersToDrop` (`KismetMathLibrary.RandomIntegerInRange` 10 20))
  (set `self.ItemTypeToDrop` (`/Game/Blueprints/C_CloudWorld.RandItemToDrop` (`self.As C Cloud World`)))
  (`self.Set classRef`))

(event `Set classRef`
  ;[1 1 1] Comment
  (switch `/Game/Blueprints/WeaponSystem/EN_Item` (`self.ItemTypeToDrop`)
    (:`NewEnumerator0`
      (set `self.DropClass` "/Game/Blueprints/WeaponSystem/Projectail/ItemDrop/Book/BP_RayBookDropProjectail.BP_RayBookDropProjectail_C"))
    (:`NewEnumerator1`
      (set `self.DropClass` "/Game/Blueprints/WeaponSystem/Projectail/ItemDrop/Book/BP_FireBookDropProjectail.BP_FireBookDropProjectail_C"))
    (:`NewEnumerator2`
      (set `self.DropClass` "/Game/Blueprints/WeaponSystem/Projectail/ItemDrop/Book/BP_GenieBookDropProjectail.BP_GenieBookDropProjectail_C"))
    (:`NewEnumerator3`
      (set `self.DropClass` "/Game/Blueprints/WeaponSystem/Projectail/ItemDrop/Book/BP_LightningBookDropProjectail.BP_LightningBookDropProjectail_C"))
    (:`NewEnumerator4`
      (set `self.DropClass` "/Game/Blueprints/WeaponSystem/Projectail/ItemDrop/Book/BP_BombBookDropProjectail.BP_BombBookDropProjectail_C"))
    (:`NewEnumerator6`
      (set `self.DropClass` "/Game/Blueprints/WeaponSystem/Projectail/ItemDrop/Weapon/BP_WandDropProjectail.BP_WandDropProjectail_C"))
    (:`NewEnumerator7`
      (set `self.DropClass` "/Game/Blueprints/WeaponSystem/Projectail/ItemDrop/Weapon/BP_StaffDropProjectail.BP_StaffDropProjectail_C"))
    (:`NewEnumerator8`
      (set `self.DropClass` "/Game/Blueprints/WeaponSystem/Projectail/ItemDrop/Weapon/BP_PistolDropProjectail.BP_PistolDropProjectail_C"))
    (:`NewEnumerator10`
      (set `self.DropClass` "/Game/Blueprints/WeaponSystem/Projectail/ItemDrop/Fetish/BP_AmuletDropProjectail.BP_AmuletDropProjectail_C"))
    (:`NewEnumerator11`
      (set `self.DropClass` "/Game/Blueprints/WeaponSystem/Projectail/ItemDrop/Fetish/BP_RingDropProjectail.BP_RingDropProjectail_C"))
    (:`NewEnumerator13`
      (set `self.DropClass` "/Game/Blueprints/WeaponSystem/Projectail/ItemDrop/BP_ShatterDropProjectail.BP_ShatterDropProjectail_C")
      (set `self.AmountItemsToDrop` (* (`KismetMathLibrary.RandomIntegerInRange` 10 20) 3))))
  (`self.SpawnDrop`)
  (`self.SpawnShatters`))

(event `SpawnShatters`
  (bind (_returnvalue_roll _returnvalue_pitch _returnvalue_yaw) (`KismetMathLibrary.BreakRotator` (`self.K2_GetActorRotation`)))
  (bind _shatterstodrop (`self.ShattersToDrop`))
  ;[1 1 1] Comment
  (set `self.Angle` (/ 360.0 (`KismetMathLibrary.Conv_IntToDouble` _shatterstodrop)))
  (for _index (range _shatterstodrop)
    (set `self.Index` _index)
    (bind _returnvalue (`|SpawnActorFromClass` "/Game/Blueprints/WeaponSystem/Projectail/ItemDrop/BP_ShatterDropProjectail.BP_ShatterDropProjectail_C" (`KismetMathLibrary.MakeTransform` (+ (`self.K2_GetActorLocation`) (0.0 0.0 200.0)) (`KismetMathLibrary.MakeRotator` _returnvalue_yaw -90.0 (+ _returnvalue_roll (* (`self.Index`) (`self.Angle`)) (`KismetMathLibrary.RandomFloatInRange` -180.0 180.0)))) "AlwaysSpawn" "OverrideRootScale" null null))
    (bind _projectilemovement (`/Game/Blueprints/WeaponSystem/Projectail/BP_projectailParent.ProjectileMovement` _returnvalue))
    (set `ProjectileMovementComponent.InitialSpeed` (* (`KismetMathLibrary.RandomFloatInRange` 0.7 1.3) 800.0) _projectilemovement)
    (bind _initialspeed (`ProjectileMovementComponent.InitialSpeed` _projectilemovement))
    (`ProjectileMovementComponent.SetVelocityInLocalSpace` _projectilemovement (`KismetMathLibrary.MakeVector` (* _initialspeed -1.0) 0.0 (* _initialspeed (`KismetMathLibrary.RandomFloatInRange` 0.05 0.3))))))

(event `SpawnDrop`
  (bind (_returnvalue_roll _returnvalue_pitch _returnvalue_yaw) (`KismetMathLibrary.BreakRotator` (`self.K2_GetActorRotation`)))
  (bind _amountitemstodrop (`self.AmountItemsToDrop`))
  ;[1 1 1] SpawnShatters hehe boy
  (set `self.Angle` (/ 360.0 (`KismetMathLibrary.Conv_IntToDouble` _amountitemstodrop)))
  (for _index (range _amountitemstodrop)
    (set `self.Index` _index)
    (bind _returnvalue (`|SpawnActorFromClass` (`self.DropClass`) (`KismetMathLibrary.MakeTransform` (+ (`self.K2_GetActorLocation`) (0.0 0.0 200.0)) (`KismetMathLibrary.MakeRotator` _returnvalue_yaw -90.0 (+ _returnvalue_roll (* (`self.Index`) (`self.Angle`)) (`KismetMathLibrary.RandomFloatInRange` -180.0 180.0)))) "AlwaysSpawn" "OverrideRootScale" null null))
    (bind _projectilemovement (`/Game/Blueprints/WeaponSystem/Projectail/BP_projectailParent.ProjectileMovement` _returnvalue))
    (set `ProjectileMovementComponent.InitialSpeed` (* (`KismetMathLibrary.RandomFloatInRange` 0.7 1.3) 1000.0) _projectilemovement)
    (bind _initialspeed (`ProjectileMovementComponent.InitialSpeed` _projectilemovement))
    (`ProjectileMovementComponent.SetVelocityInLocalSpace` _projectilemovement (`KismetMathLibrary.MakeVector` (* _initialspeed -1.0) 0.0 (* _initialspeed (`KismetMathLibrary.RandomFloatInRange` 0.0 0.15))))))

(fn `UserConstructionScript`)