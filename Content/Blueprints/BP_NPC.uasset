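; BP_NPC is an interactable NPC that moves the player into a dialog view.
; On BeginPlay it caches the cloud-world controller and player character, then sets the name text on its overlap widget.
; Interact blends to the NPC camera, teleports the player to an offset facing the NPC, and switches the controller to dialog after the blend delay.
; ShowText toggles the widget's visibility and swaps between two idle animations.
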(event `self.ReceiveBeginPlay`
  ;[0.1191 1 0] Comment
  (bind _asc_cloud_world (cast `/Game/Blueprints/C_CloudWorld` (`GameplayStatics.GetPlayerController` 0)))
  (set `self.As C Cloud World` _asc_cloud_world)
  (bind _asbp_main_character_cw (cast `/Game/Blueprints/BP_MainCharacterCW` (`GameplayStatics.GetPlayerCharacter` 0)))
  (set `self.As BP Main Character CW` _asbp_main_character_cw)
  (bind _aswb_item_widget (cast `/Game/Blueprints/Widgets/PopUp/WB_ItemWidget` (`WidgetComponent.GetWidget` (`self.OverlapWidget`))))
  (bind _output_get (set `self.As WB Item Widget` _aswb_item_widget))
  (`TextBlock.SetText` (`/Game/Blueprints/Widgets/PopUp/WB_ItemWidget.ItemName` _output_get) (`self.Text`)))

(event `/Game/Blueprints/I_Interactable.Interact`
  (bind _returnvalue (`self.K2_GetActorLocation`))
  (bind (_locationtochar_x _locationtochar_y _locationtochar_z) (`KismetMathLibrary.BreakVector` (`self.LocationToChar`)))
  (bind _as_c_cloud_world (`self.As C Cloud World`))
  (bind _returnvalue_2 (+ (`KismetMathLibrary.MakeVector` (* -1 _locationtochar_y) _locationtochar_x _locationtochar_z) _returnvalue))
  ;[1 1 1] Переходим в меню диалога
  (`PlayerController.SetViewTargetWithBlend` _as_c_cloud_world (`ActorComponent.GetOwner` (`self.NPCCamera`)) 2.0 "VTBlend_Linear" 0.0 false)
  (`self.K2_SetActorLocation` (`self.As BP Main Character CW`) _returnvalue_2 false false)
  (`self.K2_SetActorRotation` (`self.As BP Main Character CW`) (`KismetMathLibrary.FindLookAtRotation` _returnvalue_2 _returnvalue) false)
  (`SkeletalMeshComponent.PlayAnimation` (`self.NPC_SceletalMesh`) "/Game/models/NPC/anim/AN_NPC_Idle1.AN_NPC_Idle1" true)
  (`KismetSystemLibrary.Delay` 2.0)
  (`/Game/Blueprints/C_CloudWorld.SwitchToDialog` _as_c_cloud_world))

(event `/Game/Blueprints/I_Interactable.ShowText`
  (params (SetHidden :type Boolean) (MainCharRef :type "/Game/Blueprints/BP_MainCharacterCW Object Reference"))
  (bind _npc_sceletalmesh (`self.NPC_SceletalMesh`))
  ;[1 1 1] Comment
  (`SceneComponent.SetHiddenInGame` (`self.OverlapWidget`) SetHidden false)
  (if SetHidden
    (`SkeletalMeshComponent.PlayAnimation` _npc_sceletalmesh "/Game/models/NPC/anim/AN_NPC_Idle2.AN_NPC_Idle2" true)
    (else
      (`SkeletalMeshComponent.PlayAnimation` _npc_sceletalmesh "/Game/models/NPC/anim/AN_NPC_Idle1.AN_NPC_Idle1" true))))

(fn `UserConstructionScript`)