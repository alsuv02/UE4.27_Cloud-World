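; Top-down player character with WASD movement, cursor aiming, health, regenerating mana, and swappable weapons, spell books and fetishes.
; Each tick a cursor trace sets the shoot direction and turns a spring-arm marker, while shoot input is forwarded to the current weapon actor.
; Debug keys lazily spawn and attach weapon and book actors on first use, then swap current references.
; Damage leads to death, which hides the mesh and blocks movement and firing.
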(event `InputAxis|MoveForward`
  (params (AxisValue :type "Float (single-precision)"))
  ;[0.6949 0 1] Inputs
  (if (not (`self.IsDead`))
    (`self.MoveWS` AxisValue)))

(event `InputAxis|MoveRight`
  (params (AxisValue :type "Float (single-precision)"))
  ;[0.6949 0 1] Inputs
  (if (not (`self.IsDead`))
    (`self.MoveAD` AxisValue)))

(event `InputAction|Shoot`
  (params (Key :type "Key Structure"))
  (bind _currentweaponref (`self.CurrentWeaponRef`))
  ;[0.6949 0 1] Inputs
  ;;[1 1 1] Comment
  (:`Pressed`
    (if (not (`self.IsDead`))
      (`/Game/Blueprints/WeaponSystem/BP_DadWeapon.Shoot` _currentweaponref)))
  (:`Released`
    (`/Game/Blueprints/WeaponSystem/BP_DadWeapon.BurstShootStop` _currentweaponref)))

(event `BurstShootPresed`
  ;[1 1 1] BurstShoot
  (bind _returnvalue (`KismetSystemLibrary.K2_SetTimerDelegate` (`|CreateDelegate` :!event `Shoot`) (`self.Delta Seconds`) true)))

(event `BurstShootReleased`
  ;[1 1 1] BurstShoot
  (`KismetSystemLibrary.K2_ClearAndInvalidateTimerHandle` (stale `BurstShootPresed` _returnvalue)))

(event `InputAction|bURSTShoot`
  (params (Key :type "Key Structure"))
  ;[0.6949 0 1] Inputs
)

(event `Shoot`
  (bind (_shootrotation_roll _shootrotation_pitch _shootrotation_yaw) (`KismetMathLibrary.BreakRotator` (`self.ShootRotation`)))
  ;[1 1 1] Shoot
  ;;[1 1 1] Прошу не обращать внимание на эту чёрную магию, она была сделана путём кровавых жертвоприношений и демонического вмешательства.
  (`|SpawnActorFromClass` "/Game/Blueprints/BP_Arrow.BP_Arrow_C" (`KismetMathLibrary.MakeTransform` (+ (`self.K2_GetActorLocation`) (* (`self.ShootVector`) 120.0)) (`KismetMathLibrary.MakeRotator` _shootrotation_yaw -90.0 _shootrotation_roll) (0.2 0.2 0.2)) "Undefined" "OverrideRootScale" null null))

(event `MoveWS`
  (params (Forward :type "Float (double-precision)"))
  ;[1 1 1] Перемещение на wasd
  (`self.AddMovementInput` (`KismetMathLibrary.GetForwardVector` (`KismetMathLibrary.MakeRotator` 0.0 0.0 (.yaw (`self.GetControlRotation`)))) Forward))

(event `MoveAD`
  (params (Right :type "Float (double-precision)"))
  ;[1 1 1] Перемещение на wasd
  (`self.AddMovementInput` (`KismetMathLibrary.GetRightVector` (`KismetMathLibrary.MakeRotator` 0.0 0.0 (.yaw (`self.GetControlRotation`)))) Right))

(event `Death`
  ;[0 0 0] Смерть
  (`KismetSystemLibrary.PrintString` "ПОТРАЧЕНО!!!" true true (struct :`R` 1.0 :`B` 0.032746 :`A` 1.0) 10000.0)
  (set `self.IsDead` true)
  (`SceneComponent.SetVisibility` (`self.Mesh`) false false))

(event `self.ReceiveBeginPlay`
  ;[0.05317 1 0] Бегин плей
  (`self.CameraActivation`)
  (`self.GetRefs`)
  (`self.SetCurrentItemToNone`))

(event `self.ReceiveAnyDamage`
  (params (Damage :type "Float (single-precision)") (DamageType :type "DamageType Object Reference") (InstigatedBy :type "Controller Object Reference") (DamageCauser :type "Actor Object Reference"))
  (bind _returnvalue (- (`self.CurrentHealth`) Damage))
  ;[1 1 1] Получаем урон
  (if (<= _returnvalue 0.0)
    (`self.Death`)
    (else
      (set `self.CurrentHealth` _returnvalue))))

(event `self.ReceiveTick`
  (params (DeltaSeconds :type "Float (single-precision)"))
  ;[0.1732 1 0] TICK
  (set `self.Delta Seconds` DeltaSeconds)
  (`self.ConeRotate`)
  (`self.ManaRegeneration`))

(event `CameraActivation`
  ;[0 1 0.66] Эвенты бегин плей
  (`ActorComponent.Activate` (`self.Camera1`) false))

(event `ManaRegeneration`
  (set `self.CurrentMana` (+ (* (+ (/ (`self.CurrentMana`) (`self.MaxMana`)) 0.1) (`self.Delta Seconds`) (`self.ManaRegenSpeed/sec`)) (`self.CurrentMana`))))

(event `ConeRotate`
  (bind _returnvalue (`self.K2_GetActorLocation`))
  (bind (_bblockinghit _binitialoverlap _time _distance _location) (`GameplayStatics.BreakHitResult` (`PlayerController.GetHitResultUnderCursorByChannel` (`self.As Top Down Controller`) "TraceTypeQuery1" true)))
  (bind _returnvalue_2 (`KismetMathLibrary.GetDirectionUnitVector` _returnvalue _location))
  (bind (_returnvalue_roll _returnvalue_pitch _returnvalue_yaw) (`KismetMathLibrary.BreakRotator` (`KismetMathLibrary.MakeRotFromX` _returnvalue_2)))
  ;[0 1 0.5172] Лайн трейс для марки направления (конус)
  (set `self.MousePosition` _location)
  (if (< (`KismetMathLibrary.VSize` (- _location _returnvalue)) 1000.0)
    (set `self.Can Shoot` false)
    (else
      (set `self.Can Shoot` true)))
  (set `self.ShootVector` _returnvalue_2)
  (bind _output_get (set `self.ShootRotation` (`KismetMathLibrary.MakeRotator` _returnvalue_roll _returnvalue_pitch _returnvalue_yaw)))
  (`SceneComponent.K2_SetWorldRotation` (`self.SpringArmMark`) (`KismetMathLibrary.MakeRotator` 0.0 0.0 (+ (.yaw _output_get) 180.0)) false false))

(event `GetRefs`
  ;[0 1 0.66] Эвенты бегин плей
  (bind _asc_cloud_world (cast `/Game/Blueprints/C_CloudWorld` (`GameplayStatics.GetPlayerController` 0)))
  (set `self.As Top Down Controller` _asc_cloud_world))

(event `SetCurrentItemToNone`
  ;[0 1 0.66] Эвенты бегин плей
  (bind _returnvalue (`|SpawnActorFromClass` "/Game/Blueprints/WeaponSystem/WeaponChild/BP_ChildNoWeapon.BP_ChildNoWeapon_C" (`KismetMathLibrary.MakeTransform` (`self.K2_GetActorLocation`)) "Undefined" "OverrideRootScale" null null))
  (set `self.NoneWeaponRef` _returnvalue)
  (set `self.CurrentWeaponRef` _returnvalue)
  (`self.K2_AttachToActor` _returnvalue self "None" "KeepRelative" "KeepRelative" "KeepRelative" true)
  (bind _returnvalue_2 (`|SpawnActorFromClass` "/Game/Blueprints/WeaponSystem/BookChild/BP_ChildNoBook.BP_ChildNoBook_C" (`KismetMathLibrary.MakeTransform` (`self.K2_GetActorLocation`)) "Undefined" "OverrideRootScale" null null))
  (set `self.NoneBookRef` _returnvalue_2)
  (set `self.CurrentBookRef` _returnvalue_2)
  (`self.K2_AttachToActor` _returnvalue_2 self "None" "KeepRelative" "KeepRelative" "KeepRelative" true)
  (bind _returnvalue_3 (`|SpawnActorFromClass` "/Game/Blueprints/WeaponSystem/FetishChild/BP_ChildNoFetish.BP_ChildNoFetish_C" (`KismetMathLibrary.MakeTransform` (`self.K2_GetActorLocation`)) "Undefined" "OverrideRootScale" null null))
  (set `self.NoneFetishRef` _returnvalue_3)
  (set `self.CurrentFetishRef` _returnvalue_3)
  (`self.K2_AttachToActor` _returnvalue_3 self "None" "KeepRelative" "KeepRelative" "KeepRelative" true))

(event `Key|R`
  (params (Key :type "Key Structure"))
  ;[1 0.9657 0] Суррогат смены оружия
  ;;[1 1 1] Переключаемся на стандартное "без оружия"
  (:`Pressed`
    (if (not (== (`self.CurrentWeaponRef`) (`self.NoneWeaponRef`)))
      (bind _output_get (set `self.CurrentWeaponRef` (`self.NoneWeaponRef`)))
      (`KismetSystemLibrary.PrintString` (`KismetSystemLibrary.GetDisplayName` _output_get)))))

(event `Key|F10`
  (params (Key :type "Key Structure"))
  ;[1 0.8916 0] Comment
  ;;[1 1 1] Переключаемся на стандартное "без фетиша"
  (:`Pressed`
    (if (not (== (`self.NoneFetishRef`) (`self.CurrentFetishRef`)))
      (bind _output_get (set `self.CurrentFetishRef` (`self.NoneFetishRef`)))
      (`KismetSystemLibrary.PrintString` (`KismetSystemLibrary.GetDisplayName` _output_get)))))

(event `Key|One`
  (params (Key :type "Key Structure"))
  ;[1 0.9309 0] Суррогат смены книг
  ;;[1 1 1] Переключаемся на стандартное "без книги"
  (:`Pressed`
    (bind _output_get (set `self.CurrentBookRef` (`self.NoneBookRef`)))
    (`KismetSystemLibrary.PrintString` (`KismetSystemLibrary.GetDisplayName` _output_get))
    (set `self.EN_BookCurrent` "NewEnumerator5")))

(event `Key|T`
  (params (Key :type "Key Structure"))
  ;[1 0.9657 0] Суррогат смены оружия
  ;;[1 1 1] Устанавливаем оружие wand
  (:`Pressed`
    (if (`self.IsFirstWandChange`)
      (set `self.IsFirstWandChange` false)
      (bind _returnvalue (`|SpawnActorFromClass` "/Game/Blueprints/WeaponSystem/WeaponChild/BP_ChildWand.BP_ChildWand_C" (`KismetMathLibrary.MakeTransform` (`self.K2_GetActorLocation`)) "Undefined" "OverrideRootScale" null null))
      (`self.K2_AttachToActor` _returnvalue self "None" "KeepRelative" "KeepRelative" "KeepRelative" true)
      (bind _output_get (set `self.WandRef` _returnvalue))
      (bind _output_get_2 (set `self.CurrentWeaponRef` _output_get :!label _label))
      (`KismetSystemLibrary.PrintString` (`KismetSystemLibrary.GetDisplayName` _output_get_2))
      (elif (not (== (`self.CurrentWeaponRef`) (`self.WandRef`)))
        (goto _label)))))

(event `Key|F11`
  (params (Key :type "Key Structure"))
  ;[1 0.8916 0] Comment
  ;;[1 1 1] Устанавливаем оружие wand
  (:`Pressed`
    (if false
      (set `self.IsFirstWandChange` false)
      (bind _returnvalue (`|SpawnActorFromClass` "/Game/Blueprints/WeaponSystem/WeaponChild/BP_ChildWand.BP_ChildWand_C" (`KismetMathLibrary.MakeTransform` (`self.K2_GetActorLocation`)) "Undefined" "OverrideRootScale" null null))
      (`self.K2_AttachToActor` _returnvalue self "None" "KeepRelative" "KeepRelative" "KeepRelative" true)
      (bind _output_get (set `self.WandRef` _returnvalue)))
    (bind _output_get_2 (set `self.CurrentWeaponRef` _output_get))
    (`KismetSystemLibrary.PrintString` (`KismetSystemLibrary.GetDisplayName` _output_get_2))))

(event `Key|Two`
  (params (Key :type "Key Structure"))
  ;[1 0.9309 0] Суррогат смены книг
  ;;[1 1 1] Устанавливаем книгу Рэй
  (:`Pressed`
    (if (`self.IsFirstRayChange`)
      (set `self.IsFirstRayChange` false)
      (bind _returnvalue (`|SpawnActorFromClass` "/Game/Blueprints/WeaponSystem/BookChild/BP_ChildRayBook.BP_ChildRayBook_C" (`KismetMathLibrary.MakeTransform` (`self.K2_GetActorLocation`)) "Undefined" "OverrideRootScale" null null))
      (`self.K2_AttachToActor` _returnvalue self "None" "KeepRelative" "KeepRelative" "KeepRelative" true)
      (bind _output_get (set `self.RayBookRef` _returnvalue))
      (bind _output_get_2 (set `self.CurrentBookRef` _output_get :!label _label_2))
      (`KismetSystemLibrary.PrintString` (`KismetSystemLibrary.GetDisplayName` _output_get_2))
      (set `self.EN_BookCurrent` "NewEnumerator0")
      (elif (not (== (`self.CurrentBookRef`) (`self.RayBookRef`)))
        (goto _label_2)))))

(event `Key|Three`
  (params (Key :type "Key Structure"))
  ;[1 0.9309 0] Суррогат смены книг
  ;;[1 1 1] Переключаемся на огонь
  (:`Pressed`
    (if (`self.IsFirstFireChange`)
      (set `self.IsFirstFireChange` false)
      (bind _returnvalue (`|SpawnActorFromClass` "/Game/Blueprints/WeaponSystem/BookChild/BP_ChildFireBook.BP_ChildFireBook_C" (`KismetMathLibrary.MakeTransform` (`self.K2_GetActorLocation`)) "Undefined" "OverrideRootScale" null null))
      (`self.K2_AttachToActor` _returnvalue self "None" "KeepRelative" "KeepRelative" "KeepRelative" true)
      (bind _output_get (set `self.FireBookRef` _returnvalue))
      (bind _output_get_2 (set `self.CurrentBookRef` _output_get :!label _label_3))
      (`KismetSystemLibrary.PrintString` (`KismetSystemLibrary.GetDisplayName` _output_get_2))
      (set `self.EN_BookCurrent` "NewEnumerator1")
      (elif (not (== (`self.CurrentBookRef`) (`self.FireBookRef`)))
        (goto _label_3)))))

(event `Key|Y`
  (params (Key :type "Key Structure"))
  ;[1 0.9657 0] Суррогат смены оружия
  ;;[1 1 1] Устанавливаем оружие staff
  (:`Pressed`
    (if (`self.IsFirstStaffChange`)
      (set `self.IsFirstStaffChange` false)
      (bind _returnvalue (`|SpawnActorFromClass` "/Game/Blueprints/WeaponSystem/WeaponChild/BP_ChildStaff.BP_ChildStaff_C" (`KismetMathLibrary.MakeTransform` (`self.K2_GetActorLocation`)) "Undefined" "OverrideRootScale" null null))
      (`self.K2_AttachToActor` _returnvalue self "None" "KeepRelative" "KeepRelative" "KeepRelative" true)
      (bind _output_get (set `self.StaffRef` _returnvalue))
      (bind _output_get_2 (set `self.CurrentWeaponRef` _output_get :!label _label_4))
      (`KismetSystemLibrary.PrintString` (`KismetSystemLibrary.GetDisplayName` _output_get_2))
      (elif (not (== (`self.CurrentWeaponRef`) (`self.StaffRef`)))
        (goto _label_4)))))

(event `Key|F12`
  (params (Key :type "Key Structure"))
  ;[1 0.8916 0] Comment
  ;;[1 1 1] Устанавливаем оружие wand
  (:`Pressed`
    (if false
      (set `self.IsFirstWandChange` false)
      (bind _returnvalue (`|SpawnActorFromClass` "/Game/Blueprints/WeaponSystem/WeaponChild/BP_ChildWand.BP_ChildWand_C" (`KismetMathLibrary.MakeTransform` (`self.K2_GetActorLocation`)) "Undefined" "OverrideRootScale" null null))
      (`self.K2_AttachToActor` _returnvalue self "None" "KeepRelative" "KeepRelative" "KeepRelative" true)
      (bind _output_get (set `self.WandRef` _returnvalue)))
    (bind _output_get_2 (set `self.CurrentWeaponRef` _output_get))
    (`KismetSystemLibrary.PrintString` (`KismetSystemLibrary.GetDisplayName` _output_get_2))))

(event `Key|Four`
  (params (Key :type "Key Structure"))
  ;[1 0.9309 0] Суррогат смены книг
  ;;[1 1 1] Переключаемся на джинни
  (:`Pressed`
    (if (`self.IsFirstGenieChoose`)
      (set `self.IsFirstGenieChoose` false)
      (bind _returnvalue (`|SpawnActorFromClass` "/Game/Blueprints/WeaponSystem/BookChild/BP_ChildGenieBook.BP_ChildGenieBook_C" (`KismetMathLibrary.MakeTransform` (`self.K2_GetActorLocation`)) "Undefined" "OverrideRootScale" null null))
      (`self.K2_AttachToActor` _returnvalue self "None" "KeepRelative" "KeepRelative" "KeepRelative" true)
      (bind _output_get (set `self.GenieBookRef` _returnvalue))
      (bind _output_get_2 (set `self.CurrentBookRef` _output_get :!label _label_5))
      (`KismetSystemLibrary.PrintString` (`KismetSystemLibrary.GetDisplayName` _output_get_2))
      (set `self.EN_BookCurrent` "NewEnumerator2")
      (elif (not (== (`self.CurrentBookRef`) (`self.GenieBookRef`)))
        (goto _label_5)))))

(event `Key|U`
  (params (Key :type "Key Structure"))
  ;[1 0.9657 0] Суррогат смены оружия
  ;;[1 1 1] Устанавливаем оружие pistol
  (:`Pressed`
    (if (`self.IsFirstPistolChange`)
      (set `self.IsFirstPistolChange` false)
      (bind _returnvalue (`|SpawnActorFromClass` "/Game/Blueprints/WeaponSystem/WeaponChild/BP_ChildPistol.BP_ChildPistol_C" (`KismetMathLibrary.MakeTransform` (`self.K2_GetActorLocation`)) "Undefined" "OverrideRootScale" null null))
      (`self.K2_AttachToActor` _returnvalue self "None" "KeepRelative" "KeepRelative" "KeepRelative" true)
      (bind _output_get (set `self.PistolRef` _returnvalue))
      (bind _output_get_2 (set `self.CurrentWeaponRef` _output_get :!label _label_6))
      (`KismetSystemLibrary.PrintString` (`KismetSystemLibrary.GetDisplayName` _output_get_2))
      (elif (not (== (`self.CurrentWeaponRef`) (`self.PistolRef`)))
        (goto _label_6)))))

(event `Key|Five`
  (params (Key :type "Key Structure"))
  ;[1 0.9309 0] Суррогат смены книг
  ;;[1 1 1] Переключаемся на молнию
  (:`Pressed`
    (if (`self.IsFirstLightningChange`)
      (set `self.IsFirstLightningChange` false)
      (bind _returnvalue (`|SpawnActorFromClass` "/Game/Blueprints/WeaponSystem/BookChild/BP_ChildLightningBook.BP_ChildLightningBook_C" (`KismetMathLibrary.MakeTransform` (`self.K2_GetActorLocation`)) "Undefined" "OverrideRootScale" null null))
      (`self.K2_AttachToActor` _returnvalue self "None" "KeepRelative" "KeepRelative" "KeepRelative" true)
      (bind _output_get (set `self.LigtningBookRef` _returnvalue))
      (bind _output_get_2 (set `self.CurrentBookRef` _output_get :!label _label_7))
      (`KismetSystemLibrary.PrintString` (`KismetSystemLibrary.GetDisplayName` _output_get_2))
      (set `self.EN_BookCurrent` "NewEnumerator3")
      (elif (not (== (`self.CurrentBookRef`) (`self.LigtningBookRef`)))
        (goto _label_7)))))

(event `Key|Six`
  (params (Key :type "Key Structure"))
  ;[1 0.9309 0] Суррогат смены книг
  ;;[1 1 1] Переключаемся на бомбочку
  (:`Pressed`
    (if (`self.IsFirstBombChange`)
      (set `self.IsFirstBombChange` false)
      (bind _returnvalue (`|SpawnActorFromClass` "/Game/Blueprints/WeaponSystem/BookChild/BP_ChildBombBook.BP_ChildBombBook_C" (`KismetMathLibrary.MakeTransform` (`self.K2_GetActorLocation`)) "Undefined" "OverrideRootScale" null null))
      (`self.K2_AttachToActor` _returnvalue self "None" "KeepRelative" "KeepRelative" "KeepRelative" true)
      (bind _output_get (set `self.BombBookRef` _returnvalue))
      (bind _output_get_2 (set `self.CurrentBookRef` _output_get :!label _label_8))
      (`KismetSystemLibrary.PrintString` (`KismetSystemLibrary.GetDisplayName` _output_get_2))
      (set `self.EN_BookCurrent` "NewEnumerator4")
      (elif (not (== (`self.CurrentBookRef`) (`self.BombBookRef`)))
        (goto _label_8)))))

(fn `UserConstructionScript`
  (bind _output_get (set `self.MaxHealth` 100.0))
  (set `self.CurrentHealth` _output_get)
  (bind _output_get_2 (set `self.MaxMana` 100.0))
  (set `self.CurrentMana` _output_get_2))