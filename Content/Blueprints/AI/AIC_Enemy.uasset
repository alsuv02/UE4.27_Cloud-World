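; AIC_Enemy is the AI controller for enemies, running the BT_Enemy behavior tree on BeginPlay and clearing the TargetActor blackboard key.
; AI Perception updates write the sensed actor to TargetActor, or clear the key when a stimulus is lost.
; Each update briefly draws a debug sphere around the pawn, with a larger red one on loss.
; Any perceived actor becomes the target, with no filtering by type or team in the graph.
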(event `self.ReceiveBeginPlay`
  (`self.RunBehaviorTree` "/Game/Blueprints/AI/BT_Enemy.BT_Enemy")
  (`BlackboardComponent.ClearValue` (`self.Blackboard`) "TargetActor"))

(event `self.AIPerception.OnTargetPerceptionUpdated`
  (params (Actor :type "Actor Object Reference") (Stimulus :type "AIStimulus Structure"))
  ;[1 1 1] Увидел или потерял?
  (if (`.bSuccessfullySensed` (break `AIStimulus` Stimulus))
    ;[1 1 1] отрисовка сфер
    (`KismetSystemLibrary.DrawDebugSphere` (`self.K2_GetActorLocation` (`self.K2_GetPawn` self)) 500.0 12 (struct :`R` 1.0 :`G` 1.0 :`B` 1.0 :`A` 1.0) 0.5)
    ;[1 1 1] Сетаем персонажа в доску
    (`BlackboardComponent.SetValueAsObject` (`self.Blackboard`) "TargetActor" Actor)
    (else
      (`KismetSystemLibrary.DrawDebugSphere` (`self.K2_GetActorLocation` (`self.K2_GetPawn` self)) 1000.0 12 (struct :`R` 1.0 :`A` 1.0) 0.5)
      ;[1 1 1] Очищаем значение с доски
      (`BlackboardComponent.ClearValue` (`self.Blackboard`) "TargetActor"))))

(fn `UserConstructionScript`)