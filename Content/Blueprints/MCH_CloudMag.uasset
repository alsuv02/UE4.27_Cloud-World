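; Player mage character for a top-down shooter, with WASD movement, cursor-aimed BP_Arrow shots and a death state that hides the mesh.
; Each Tick, ConeRotate turns the cursor hit into the shot direction and swings the spring arm to match.
; Shoot spawns an arrow along that direction; burst input runs a looping timer at frame-delta interval.
; IsDead blocks movement and firing, while CanShoot is computed from cursor distance but never checked here.
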(event `InputAxis|MoveForward`
  (params (AxisValue :type "Float (single-precision)"))
  ;[0.6949 0 1] Inputs
  (if (not (`self.IsDead`))
    (`self.MoveWS` AxisValue)))

(event `InputAxis|MoveRight`
  (params (AxisValue :type "Float (single-precision)"))
  ;[0.6949 0 1] Inputs
  (if (not (`self.IsDead`))
    (`self.MoveAD` AxisValue)))

(event `InputAction|Shoot`
  (params (Key :type "Key Structure"))
  ;[0.6949 0 1] Inputs
  (:`Pressed`
    (if (not (`self.IsDead`))
      (`self.Shoot`))))

(event `BurstShootPresed`
  ;[1 1 1] BurstShoot
  (bind _returnvalue (`KismetSystemLibrary.K2_SetTimerDelegate` (`|CreateDelegate` :!event `Shoot`) (`self.Delta Seconds`) true)))

(event `BurstShootReleased`
  ;[1 1 1] BurstShoot
  (`KismetSystemLibrary.K2_ClearAndInvalidateTimerHandle` (stale `BurstShootPresed` _returnvalue)))

(event `InputAction|bURSTShoot`
  (params (Key :type "Key Structure"))
  (bind _isdead (`self.IsDead`))
  ;[0.6949 0 1] Inputs
  (:`Pressed`
    (if (not _isdead)
      (`self.BurstShootPresed`)))
  (:`Released`
    (if _isdead
      (`/Engine/EditorBlueprintResources/StandardMacros.DoOnce` false
        (:`Completed`
          _)))
    (`self.BurstShootReleased`)))

(event `Shoot`
  (bind (_shootrotation_roll _shootrotation_pitch _shootrotation_yaw) (`KismetMathLibrary.BreakRotator` (`self.ShootRotation`)))
  ;[1 1 1] Shoot
  (`|SpawnActorFromClass` "/Game/Blueprints/BP_Arrow.BP_Arrow_C" (`KismetMathLibrary.MakeTransform` (+ (`self.K2_GetActorLocation`) (* (`self.ShootVector`) 120.0)) (`KismetMathLibrary.MakeRotator` _shootrotation_yaw -90.0 _shootrotation_roll) (0.2 0.2 0.2)) "Undefined" "OverrideRootScale" null null))

(event `MoveWS`
  (params (Forward :type "Float (double-precision)"))
  ;[1 1 1] Перемещение на wasd
  (`self.AddMovementInput` (`KismetMathLibrary.GetForwardVector` (`KismetMathLibrary.MakeRotator` 0.0 0.0 (.yaw (`self.GetControlRotation`)))) Forward))

(event `self.ReceiveActorBeginOverlap`
  (params (OtherActor :type "Actor Object Reference"))
  ;[0.6949 0 1] Inputs
  (if (`self.IsDead`)
    _))

(event `MoveAD`
  (params (Right :type "Float (double-precision)"))
  ;[1 1 1] Перемещение на wasd
  (`self.AddMovementInput` (`KismetMathLibrary.GetRightVector` (`KismetMathLibrary.MakeRotator` 0.0 0.0 (.yaw (`self.GetControlRotation`)))) Right))

(event `Death`
  ;[0 0 0] Смерть
  (`KismetSystemLibrary.PrintString` "ПОТРАЧЕНО!!!" true true (struct :`R` 1.0 :`B` 0.032746 :`A` 1.0) 10000.0)
  (set `self.IsDead` true)
  (`SceneComponent.SetVisibility` (`self.Mesh`) false false))

(event `self.ReceiveBeginPlay`
  ;[0.05317 1 0] Бегин плей
  (`self.CameraActivation`)
  (`self.GetRefs`)
  (`self.SetActorsToIgnore`))

(event `self.ReceiveTick`
  (params (DeltaSeconds :type "Float (single-precision)"))
  ;[0.1732 1 0] Comment
  (set `self.Delta Seconds` DeltaSeconds)
  (`self.ConeRotate`))

(event `CameraActivation`
  ;[0 1 0.66] Эвенты бегин плей
  (`ActorComponent.Activate` (`self.Camera1`) false))

(event `ConeRotate`
  (bind _returnvalue (`self.K2_GetActorLocation`))
  (bind (_bblockinghit _binitialoverlap _time _distance _location) (`GameplayStatics.BreakHitResult` (`PlayerController.GetHitResultUnderCursorByChannel` (`self.As Top Down Controller`) "TraceTypeQuery1" true)))
  (bind _returnvalue_2 (`KismetMathLibrary.GetDirectionUnitVector` _returnvalue _location))
  (bind (_returnvalue_roll _returnvalue_pitch _returnvalue_yaw) (`KismetMathLibrary.BreakRotator` (`KismetMathLibrary.MakeRotFromX` _returnvalue_2)))
  ;[0 1 0.5172] Лайн трейс для марки направления (конус)
  (if (< (`KismetMathLibrary.VSize` (- _location _returnvalue)) 1000.0)
    (set `self.Can Shoot` false)
    (else
      (set `self.Can Shoot` true)))
  (set `self.ShootVector` _returnvalue_2)
  (bind _output_get (set `self.ShootRotation` (`KismetMathLibrary.MakeRotator` _returnvalue_roll _returnvalue_pitch _returnvalue_yaw)))
  (`SceneComponent.K2_SetWorldRotation` (`self.SpringArm`) (`KismetMathLibrary.MakeRotator` 0.0 0.0 (+ (.yaw _output_get) 180.0)) false false)
  (`SceneComponent.K2_SetWorldRotation` (`self.SpringArm`) (`KismetMathLibrary.MakeRotator` 0.0 0.0 (+ (.yaw _output_get) 180.0)) false false))

(event `GetRefs`
  ;[0 1 0.66] Эвенты бегин плей
  (bind _asc_cloud_world (cast `/Game/Blueprints/C_CloudWorld` (`GameplayStatics.GetPlayerController` 0)))
  (set `self.As Top Down Controller` _asc_cloud_world))

(event `SetActorsToIgnore`
  ;[0 1 0.66] Эвенты бегин плей
  ;;[1 0.04355 0] Comment
  (bind _outactors (`GameplayStatics.GetAllActorsOfClass` "/Game/Blueprints/BP_Cube.BP_Cube_C"))
  (set `self.Actors to Ignore` _outactors))

(fn `UserConstructionScript`)