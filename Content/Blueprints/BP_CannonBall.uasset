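; BP_CannonBall is a projectile actor that damages CH_enemy actors and keeps flying after hitting them.
; All logic runs from the projectile movement's stop event.
; On an enemy hit it applies damage, reassigns the Sphere as updated component to restart movement, and sets local-space velocity from the actor's forward vector.
; Any other impact destroys it after a zero-length delay.
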(event `self.ProjectileMovement.OnProjectileStop`
  (params (ImpactResult :type "HitResult Structure (by ref)"))
  (bind _projectilemovement (`self.ProjectileMovement`))
  (bind `_asсh_enemy` (cast `/Game/Blueprints/СH_enemy` (`.HitActor` (`GameplayStatics.BreakHitResult` ImpactResult)))
    (:`then`
      (`GameplayStatics.ApplyDamage` `_asсh_enemy` 1.0)
      (`MovementComponent.SetUpdatedComponent` _projectilemovement (`self.Sphere`))
      (`ProjectileMovementComponent.SetVelocityInLocalSpace` _projectilemovement (* (`self.GetActorForwardVector`) 1000.0)))
    (:`CastFailed`
      (`KismetSystemLibrary.Delay` 0.0)
      (`self.K2_DestroyActor`))))

(fn `UserConstructionScript`)