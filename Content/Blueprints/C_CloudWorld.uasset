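; Player controller for the cloud world that manages HUD and inventory widgets, pausing, and procedural room loading.
; LoadNewRoom derives grid coordinates from an arch's room, records them in a map, and streams MP_LoadingLevel as a coordinate-named instance offset from that arch.
; New coordinates pass through the character for the loaded room to pick up.
; An existing coordinate only prints a message, without stopping the load.
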(event `self.ReceiveBeginPlay`
  (bind _asbp_main_character_cw (cast `/Game/Blueprints/BP_MainCharacterCW` (`GameplayStatics.GetPlayerCharacter` 0)))
  (set `self.As MCH Cloud Mag` _asbp_main_character_cw)
  (bind _returnvalue (`|CreateWidget` "/Game/Blueprints/Widgets/WB_GameMain.WB_GameMain_C" self))
  (bind _output_get (set `self.WB_GameMainRef` _returnvalue))
  (`UserWidget.AddToViewport` _output_get 0)
  (bind _returnvalue_2 (`|CreateWidget` "/Game/Blueprints/Widgets/Inventory/WB_Inventory.WB_Inventory_C"))
  (set `self.WB_InventoryRef` _returnvalue_2))

(event `OnPistonWidgetsVisibiliti`
  (bind _wb_gamemainref (`self.WB_GameMainRef`))
  (`Widget.SetVisibility` (`/Game/Blueprints/Widgets/WB_GameMain.WB_Pistons` _wb_gamemainref) "Visible")
  (`Widget.SetVisibility` (`/Game/Blueprints/Widgets/WB_GameMain.WB_Pistol` _wb_gamemainref) "Visible"))

(event `Paused/Unpaused`
  (bind _isa (`/Engine/EditorBlueprintResources/StandardMacros.FlipFlop`)
    (:`A`
      _)
    (:`B`
      _))
  (`GameplayStatics.SetGamePaused` _isa))

(event `OffPistonWidgetsVisibility`
  (bind _wb_gamemainref (`self.WB_GameMainRef`))
  (`Widget.SetVisibility` (`/Game/Blueprints/Widgets/WB_GameMain.WB_Pistons` _wb_gamemainref) "Hidden")
  (`Widget.SetVisibility` (`/Game/Blueprints/Widgets/WB_GameMain.WB_Pistol` _wb_gamemainref) "Hidden"))

(event `InputAction|ToggleInventory`
  (params (Key :type "Key Structure"))
  (bind _wb_inventoryref (`self.WB_InventoryRef`))
  (:`Pressed`
    (if (not (`Widget.IsInViewport` _wb_inventoryref))
      (`self.Paused/Unpaused`)
      (`/Game/Blueprints/Widgets/Inventory/WB_Inventory.Show` _wb_inventoryref Key))))

(event `LoadNewRoom`
  (params (ArchRef :type "/Game/Maps/OneBigMap/BP_TriggerAncher Object Reference") (Type :type "/Game/Maps/OneBigMap/EN_+-xy Enum" :default "NewEnumerator0"))
  (bind _returnvalue (`KismetStringLibrary.Concat_StrStr` (`KismetStringLibrary.Conv_DoubleToString` (`self.TempX_Index`)) ";" (`KismetStringLibrary.Conv_DoubleToString` (`self.TempY_Index`))))
  ;[0 0.07486 1] вырезано
  (set `self.Arch Ref` ArchRef)
  ;;[1 1 1] Вычисляем и сетаем XY
  (`self.CalculateNewRoomIndexXY` Type)
  ;;[1 1 1] Проверяем, существует ли комнта с такими координатами.
  (`self.Check and write in Map`)
  ;;[1 1 1] Подгружаем сам уровень
  (bind _boutsuccess (`LevelStreamingDynamic.LoadLevelInstanceBySoftObjectPtr` "/Game/Maps/OneBigMap/MP_LoadingLevel.MP_LoadingLevel" (+ (`self.K2_GetActorLocation` (`self.Arch Ref`)) (select `/Game/Maps/OneBigMap/EN_+-xy` Type :`NewEnumerator0` (500.0 0.0 0.0) :`NewEnumerator1` (0.0 500.0 0.0) :`NewEnumerator2` (-500.0 0.0 0.0) :`NewEnumerator3` (0.0 -500.0 0.0) :!type "Vector Structure")) (struct) _returnvalue))
  ;;[1 1 1] Дебаг момент
  (`KismetSystemLibrary.PrintString` (`KismetStringLibrary.Concat_StrStr` " spawned Lvl " (`KismetStringLibrary.Conv_BoolToString` _boutsuccess) " " _returnvalue)))

(fn `CalculateNewRoomIndexXY`
  (params (AncherType :type "/Game/Maps/OneBigMap/EN_+-xy Enum" :default "NewEnumerator0"))
  (bind (_x _y) (`KismetMathLibrary.BreakVector2D` (`/Game/Maps/OneBigMap/BP_CoordContainer.CoordsOfMyRoom` (`/Game/Maps/OneBigMap/BP_TriggerAncher.RefToCoordsOfMyRoom` (`self.Arch Ref`)))))
  ;[1 1 1] Рассчитываем координаты новой комнаты
  (set `self.TempX_Index` (+ _x (select `/Game/Maps/OneBigMap/EN_+-xy` AncherType :`NewEnumerator0` 1.0 :`NewEnumerator2` -1.0 :!type "Float (single-precision)")))
  (set `self.TempY_Index` (+ _y (select `/Game/Maps/OneBigMap/EN_+-xy` AncherType :`NewEnumerator1` 1.0 :`NewEnumerator3` -1.0 :!type "Float (single-precision)")))
  (return))

(fn `Check and write in Map`
  (bind _returnvalue (`KismetMathLibrary.MakeVector2D` (`self.TempX_Index`) (`self.TempY_Index`)))
  ;[1 1 1] Существует ли комната с такими координатами?
  (if (`BlueprintMapLibrary.Map_Contains` (`self.MAP`) (`KismetMathLibrary.MakeVector2D` (`self.TempX_Index`) (`self.TempY_Index`)))
    (`KismetSystemLibrary.PrintString` "already exist")
    (else
      ;[1 1 1] Дополняем карту
      (`BlueprintMapLibrary.Map_Add` (`self.MAP`) _returnvalue true)
      ;[1 1 1] Кладём коорды новой комнаты в персонажа. После подгрузки комнаты актор-хранилище коорд подтянет их из персонажа.
      (set `/Game/Blueprints/BP_MainCharacterCW.RoomCoordTemp` _returnvalue (`self.As MCH Cloud Mag`))
      (return))))

(fn `UserConstructionScript`)