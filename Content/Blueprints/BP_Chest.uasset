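; Loot chest that shows its item name on a widget and, on its first interaction, hides itself and drops loot.
; GenerateItemToDrop maps the item type to a book, weapon, mascot or shard projectile class, then spawns those drops plus a random count of bonus shards.
; Both spawn loops launch projectiles in an evenly spaced ring.
; SetFence toggles visibility and collision on four fence parts while the chest is unopened.
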(event `SetFence`
  (params (SetUp :type Boolean))
  (if (`self.IsClose?`)
    (`self.SetFenceMacros` SetUp)))

(event `self.ReceiveBeginPlay`
  ;[0.09245 1 0] Comment
  (`self.SetFence` false)
  (bind _aswb_item_widget (cast `/Game/Blueprints/Widgets/PopUp/WB_ItemWidget` (`WidgetComponent.GetWidget` (`self.Widget`))))
  (set `self.WidgetRef` _aswb_item_widget)
  (`TextBlock.SetText` (`/Game/Blueprints/Widgets/PopUp/WB_ItemWidget.ItemName` _aswb_item_widget) (`self.ItemName`)))

(event `/Game/Blueprints/I_Interactable.ShowText`
  (params (SetHidden :type Boolean) (MainCharRef :type "/Game/Blueprints/BP_MainCharacterCW Object Reference"))
  ;[1 1 1] Comment
  (`SceneComponent.SetHiddenInGame` (`self.Widget`) SetHidden false))

(event `GenerateItemToDrop`
  ;[1 1 1] Comment
  (set `self.ShattersToDrop` (`KismetMathLibrary.RandomIntegerInRange` 10 20))
  (switch `/Game/Blueprints/WeaponSystem/EN_Item` (`self.ItemTypeToDrop`)
    (:`NewEnumerator0`
      (set `self.DropClass` "/Game/Blueprints/WeaponSystem/Projectail/ItemDrop/Book/BP_RayBookDropProjectail.BP_RayBookDropProjectail_C"))
    (:`NewEnumerator1`
      (set `self.DropClass` "/Game/Blueprints/WeaponSystem/Projectail/ItemDrop/Book/BP_FireBookDropProjectail.BP_FireBookDropProjectail_C"))
    (:`NewEnumerator2`
      (set `self.DropClass` "/Game/Blueprints/WeaponSystem/Projectail/ItemDrop/Book/BP_GenieBookDropProjectail.BP_GenieBookDropProjectail_C"))
    (:`NewEnumerator3`
      (set `self.DropClass` "/Game/Blueprints/WeaponSystem/Projectail/ItemDrop/Book/BP_LightningBookDropProjectail.BP_LightningBookDropProjectail_C"))
    (:`NewEnumerator4`
      (set `self.DropClass` "/Game/Blueprints/WeaponSystem/Projectail/ItemDrop/Book/BP_BombBookDropProjectail.BP_BombBookDropProjectail_C"))
    (:`NewEnumerator6`
      (set `self.DropClass` "/Game/Blueprints/WeaponSystem/Projectail/ItemDrop/Weapon/BP_WandDropProjectail.BP_WandDropProjectail_C"))
    (:`NewEnumerator7`
      (set `self.DropClass` "/Game/Blueprints/WeaponSystem/Projectail/ItemDrop/Weapon/BP_StaffDropProjectail.BP_StaffDropProjectail_C"))
    (:`NewEnumerator8`
      (set `self.DropClass` "/Game/Blueprints/WeaponSystem/Projectail/ItemDrop/Weapon/BP_PistolDropProjectail.BP_PistolDropProjectail_C"))
    (:`NewEnumerator10`
      (set `self.DropClass` "/Game/Blueprints/WeaponSystem/Projectail/ItemDrop/Fetish/BP_AmuletDropProjectail.BP_AmuletDropProjectail_C"))
    (:`NewEnumerator11`
      (set `self.DropClass` "/Game/Blueprints/WeaponSystem/Projectail/ItemDrop/Fetish/BP_RingDropProjectail.BP_RingDropProjectail_C"))
    (:`NewEnumerator13`
      (set `self.DropClass` "/Game/Blueprints/WeaponSystem/Projectail/ItemDrop/BP_ShatterDropProjectail.BP_ShatterDropProjectail_C")
      (set `self.ItemsToDrop` (* (`KismetMathLibrary.RandomIntegerInRange` 10 20) 3))))
  (`self.SpawnDrop`)
  (`self.SpawnShatters`))

(event `/Game/Blueprints/I_Interactable.Interact`
  (if (`self.IsClose?`)
    (set `self.IsClose?` false)
    ;[1 0.4162 0] Временная мера, пока актор просто прячется
    (`self.SetActorHiddenInGame` true)
    (`self.SetActorEnableCollision` false)
    (`self.GenerateItemToDrop`)))

(event `SpawnShatters`
  (bind (_returnvalue_roll _returnvalue_pitch _returnvalue_yaw) (`KismetMathLibrary.BreakRotator` (`self.K2_GetActorRotation`)))
  (bind _shatterstodrop (`self.ShattersToDrop`))
  ;[1 1 1] Comment
  (set `self.Angle` (/ 360.0 (`KismetMathLibrary.Conv_IntToDouble` _shatterstodrop)))
  (for _index (range _shatterstodrop)
    (set `self.Index` _index)
    (bind _returnvalue (`|SpawnActorFromClass` "/Game/Blueprints/WeaponSystem/Projectail/ItemDrop/BP_ShatterDropProjectail.BP_ShatterDropProjectail_C" (`KismetMathLibrary.MakeTransform` (+ (`self.K2_GetActorLocation`) (0.0 0.0 200.0)) (`KismetMathLibrary.MakeRotator` _returnvalue_yaw -90.0 (+ _returnvalue_roll (* (`self.Index`) (`self.Angle`))))) "AlwaysSpawn" "OverrideRootScale" null null))
    (bind _projectilemovement (`/Game/Blueprints/WeaponSystem/Projectail/BP_projectailParent.ProjectileMovement` _returnvalue))
    (bind _initialspeed (`ProjectileMovementComponent.InitialSpeed` _projectilemovement))
    (`ProjectileMovementComponent.SetVelocityInLocalSpace` _projectilemovement (`KismetMathLibrary.MakeVector` (* _initialspeed -1.0) 0.0 (* _initialspeed (`KismetMathLibrary.RandomFloatInRange` 0.0 0.1))))))

(event `SpawnDrop`
  (bind (_returnvalue_roll _returnvalue_pitch _returnvalue_yaw) (`KismetMathLibrary.BreakRotator` (`self.K2_GetActorRotation`)))
  (bind _itemstodrop (`self.ItemsToDrop`))
  ;[1 1 1] SpawnShatters hehe boy
  (set `self.Angle` (/ 360.0 (`KismetMathLibrary.Conv_IntToDouble` _itemstodrop)))
  (for _index (range _itemstodrop)
    (set `self.Index` _index)
    (bind _returnvalue (`|SpawnActorFromClass` (`self.DropClass`) (`KismetMathLibrary.MakeTransform` (+ (`self.K2_GetActorLocation`) (0.0 0.0 200.0)) (`KismetMathLibrary.MakeRotator` _returnvalue_yaw -90.0 (+ _returnvalue_roll (* (`self.Index`) (`self.Angle`))))) "AlwaysSpawn" "OverrideRootScale" null null))
    (bind _projectilemovement (`/Game/Blueprints/WeaponSystem/Projectail/BP_projectailParent.ProjectileMovement` _returnvalue))
    (bind _initialspeed (`ProjectileMovementComponent.InitialSpeed` _projectilemovement))
    (`ProjectileMovementComponent.SetVelocityInLocalSpace` _projectilemovement (`KismetMathLibrary.MakeVector` (* _initialspeed -1.0) 0.0 (* _initialspeed (`KismetMathLibrary.RandomFloatInRange` 0.0 0.1))))))

(fn `UserConstructionScript`)